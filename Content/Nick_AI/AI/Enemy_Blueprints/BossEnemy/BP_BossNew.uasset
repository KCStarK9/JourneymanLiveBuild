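; Boss enemy character that turns toward its AI controller's target while attacking with a launched fist, laser or melee.
; Montage notifies drive BPCEnemyAttacks for fist (hiding the hand bone) and laser; montage end reports attack end.
; Melee notifies run box traces at hand sockets, with results unused.
; Player overlap with the Box plays a one-time unpossessed intro with aura and camera shake, and applies looping timer damage until exit.
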(event `self.FireSecondFist`
  (params (AttackTarget :type "Actor Object Reference"))
  ;[1 1 1] Redundant
)

(event `self.ReceiveBeginPlay`
  (`parent.ReceiveBeginPlay`))

(event `self.ReceiveTick`
  (params (DeltaSeconds :type "Float (single-precision)"))
  ;[1 1 1] Look At player
  (if (`self.Firing Fist`)
    _
    (else
      _))
  (bind _asai_controller (cast `/Game/Nick_AI/AI/Enemy_Blueprints/AI_Controller` (`self.GetController`)))
  (if (`/Game/Nick_AI/AI/Enemy_Blueprints/AI_Controller.ISAttacking?` _asai_controller)
    (`/Engine/EditorBlueprintResources/StandardMacros.IsValid` _asai_controller
      (:`Is Valid`
        (bind (_returnvalue_roll _returnvalue_pitch _returnvalue_yaw) (`KismetMathLibrary.BreakRotator` (`KismetMathLibrary.FindLookAtRotation` (`self.K2_GetActorLocation`) (`self.K2_GetActorLocation` (`/Game/Nick_AI/AI/Enemy_Blueprints/AI_Controller.Attack Target` _asai_controller)))))
        (`self.K2_SetActorRotation` (`KismetMathLibrary.RInterpTo` (`self.K2_GetActorRotation`) (`KismetMathLibrary.MakeRotator` 0.0 0.0 _returnvalue_yaw) (`GameplayStatics.GetWorldDeltaSeconds`) (`self.Look At Rotation Speed`)))))))

(event `self.FireFirstFist`
  (params (AttackTarget :type "Actor Object Reference"))
  ;[1 1 1] Right Fist
  (bind _notifyname (`|PlayMontage` (`self.Mesh`) (`self.RightFistMontage`))
    (:`OnCompleted`
      (`self.OnAttackEnd` :!label _label)
      (`self.AttackEnd` AttackTarget)
      (`KismetSystemLibrary.Delay` 0.5)
      (`SkinnedMeshComponent.UnHideBoneByName` (`self.Mesh`) "Right_Rock_Hand"))
    (:`OnInterrupted`
      (goto _label))
    (:`OnNotifyBegin`
      (switch `name` _notifyname
        (:`Fire`
          (`SkinnedMeshComponent.HideBoneByName` (`self.Mesh`) "Right_Rock_Hand" "PBO_None")
          (bind _asai_controller (cast `/Game/Nick_AI/AI/Enemy_Blueprints/AI_Controller` (`AIBlueprintHelperLibrary.GetAIController` self)))
          (bind _attack_target (`/Game/Nick_AI/AI/Enemy_Blueprints/AI_Controller.Attack Target` _asai_controller)
            (:`then`
              (bind _returnvalue (`SkinnedMeshComponent.IsBoneHiddenByName` (`self.Mesh`) "Right_Rock_Hand"))
              (if _returnvalue
                (set `self.Look At Rotation Speed` 3.0)
                (`/Game/Nick_AI/SimpleProjectile/BPC_EnemyAttacks.LaunchFist` (`self.BPC_EnemyAttacks`) _attack_target (`SceneComponent.GetSocketTransform` (`self.Mesh`) "Fist Launch" "RTS_World"))))
            (:`else`)))))))

(event `self.FireBossLaser`
  (params (`Attack Target` :type "Actor Object Reference"))
  (bind _returnvalue (`SceneComponent.GetSocketLocation` (`self.Mesh`) "LaserREF"))
  ;[1 1 1] Fire Laser
  (`parent.FireBossLaser` `Attack Target`)
  (bind _notifyname (`|PlayMontage` (`self.Mesh`) "/Game/Nick_AI/AI/Enemy_Blueprints/BossEnemy/Animations/Montage/AM_BossLaser.AM_BossLaser" 0.5)
    (:`OnCompleted`
      (`self.OnAttackEnd` :!label _label_2)
      (`self.AttackEnd` `Attack Target`))
    (:`OnInterrupted`
      (goto _label_2))
    (:`OnNotifyBegin`
      (switch `name` _notifyname
        (:`Fire`
          (bind _asai_controller (cast `/Game/Nick_AI/AI/Enemy_Blueprints/AI_Controller` (`AIBlueprintHelperLibrary.GetAIController` self)))
          (bind _attack_target (`/Game/Nick_AI/AI/Enemy_Blueprints/AI_Controller.Attack Target` _asai_controller)
            (:`then`
              (`GameplayStatics.PlaySound2D` "/Game/Nick_AI/VFX/LaserBeam/LaserBeam.LaserBeam" 1.0 1.0 0.0 null null)
              (`KismetSystemLibrary.Delay` 0.5)
              (bind _returnvalue_2 (`self.K2_GetActorLocation` _attack_target))
              (`/Game/Nick_AI/SimpleProjectile/BPC_EnemyAttacks.FireBossLaser` (`self.BPC_EnemyAttacks`) (`KismetMathLibrary.MakeTransform` _returnvalue (`KismetMathLibrary.RInterpTo_Constant` (`KismetMathLibrary.FindLookAtRotation` _returnvalue _returnvalue_2) (`KismetMathLibrary.MakeRotFromY` _returnvalue_2) (`GameplayStatics.GetWorldDeltaSeconds`) 0.01)) _attack_target)
              (`self.K2_AttachToComponent` (`/Game/Nick_AI/SimpleProjectile/BPC_EnemyAttacks.LaserREF` (`self.BPC_EnemyAttacks`)) (`self.Mesh`) "LaserREF" "KeepWorld" "KeepWorld" "KeepWorld" true))
            (:`else`)))))))

(event `self.PrimaryAttack`
  (params (AttackTarget :type "Actor Object Reference"))
  (bind _mesh (`self.Mesh`))
  (bind _mesh_2 (`self.Mesh`))
  (bind _returnvalue (`SceneComponent.GetSocketLocation` _mesh "HitPointLEFT"))
  (bind _returnvalue_2 (`SceneComponent.GetSocketLocation` _mesh_2 "HitPointRIGHT"))
  (bind _returnvalue_3 (`SceneComponent.GetSocketRotation` _mesh "HitPointLEFT"))
  (bind _returnvalue_4 (`SceneComponent.GetSocketRotation` _mesh_2 "HitPointRIGHT"))
  (bind _returnvalue_5 (`AIBlueprintHelperLibrary.GetAIController` self))
  ;[1 1 1] Comment
  (`parent.PrimaryAttack` AttackTarget)
  (bind _notifyname (`|PlayMontage` (`self.Mesh`) (`self.MeleeMontage`))
    (:`OnCompleted`
      (`self.OnAttackEnd` :!label _label_3)
      (`self.AttackEnd` AttackTarget))
    (:`OnInterrupted`
      (goto _label_3))
    (:`OnNotifyBegin`
      (switch `name` _notifyname
        (:`LeftFist`
          (bind _asai_controller (cast `/Game/Nick_AI/AI/Enemy_Blueprints/AI_Controller` _returnvalue_5))
          (`/Game/Nick_AI/AI/Enemy_Blueprints/AI_Controller.Attack Target` _asai_controller
            (:`then`
              (`KismetSystemLibrary.BoxTraceSingleForObjects` _returnvalue (+ _returnvalue (* (`KismetMathLibrary.GetForwardVector` _returnvalue_3) 100.0)) (50.0 50.0 50.0) _returnvalue_3 (`|MakeArray` "ObjectTypeQuery3" :!type "EObjectTypeQuery Enum") false (`|MakeArray` self :!type "Actor Object Reference") "None" true (struct :`R` 1.0 :`A` 1.0) (struct :`R` 0.064528 :`G` 0.291361 :`B` 1.0 :`A` 1.0)))
            (:`else`)))
        (:`RightFist`
          (bind _asai_controller_2 (cast `/Game/Nick_AI/AI/Enemy_Blueprints/AI_Controller` _returnvalue_5))
          (`/Game/Nick_AI/AI/Enemy_Blueprints/AI_Controller.Attack Target` _asai_controller_2
            (:`then`
              (`KismetSystemLibrary.BoxTraceSingleForObjects` _returnvalue_2 (+ _returnvalue_2 (* (`KismetMathLibrary.GetForwardVector` _returnvalue_4) 100.0)) (50.0 50.0 50.0) _returnvalue_4 (`|MakeArray` "ObjectTypeQuery3" :!type "EObjectTypeQuery Enum") false (`|MakeArray` self :!type "Actor Object Reference") "None" true (struct :`R` 1.0 :`A` 1.0) (struct :`R` 0.064528 :`G` 0.291361 :`B` 1.0 :`A` 1.0)))
            (:`else`)))))))

(event `self.Box.OnComponentBeginOverlap`
  (params (OverlappedComponent :type "PrimitiveComponent Object Reference") (OtherActor :type "Actor Object Reference") (OtherComp :type "PrimitiveComponent Object Reference") (OtherBodyIndex :type Integer) (bFromSweep :type Boolean) (SweepResult :type "HitResult Structure (by ref)"))
  (if (== OtherActor (`GameplayStatics.GetPlayerCharacter` 0))
    (`|ExecutionSequence`
      (:`then_0`
        (`/Engine/EditorBlueprintResources/StandardMacros.DoOnce` false
          (:`Completed`
            (`Controller.UnPossess` (`self.GetController`))
            (bind _notifyname (`|PlayMontage` (`self.Mesh`) "/Game/Nick_AI/AI/Enemy_Blueprints/BossEnemy/Animations/Montage/AM_BossLaser.AM_BossLaser" 0.5)
              (:`OnCompleted`
                (`self.SpawnDefaultController`)
                (set `self.AIControllerClass` "/Game/Nick_AI/AI/Enemy_Blueprints/AI_Controller.AI_Controller_C"))
              (:`OnNotifyBegin`
                (switch `name` _notifyname
                  (:`Aura`
                    (`ActorComponent.Activate` (`self.Aura`) false))
                  (:`Shake`
                    (`GameplayStatics.PlayWorldCameraShake` "/Game/Nick_AI/Misc/CS_Test.CS_Test_C" (`self.K2_GetActorLocation` (`self.Gun Panda REF`)) 100.0 1500.0))))))))
      (:`then_1`
        (bind _returnvalue (`KismetSystemLibrary.K2_SetTimerDelegate` (delegate `DoDamage`) (`GameplayStatics.GetWorldDeltaSeconds`) true))
        (set `self.AuraDamageTimer` _returnvalue)))))

(event `DoDamage`
  (`GameplayStatics.ApplyDamage` (`GameplayStatics.GetPlayerCharacter` 0) (`KismetMathLibrary.RandomFloatInRange` 0.05 0.07) null self))

(event `self.Box.OnComponentEndOverlap`
  (params (OverlappedComponent :type "PrimitiveComponent Object Reference") (OtherActor :type "Actor Object Reference") (OtherComp :type "PrimitiveComponent Object Reference") (OtherBodyIndex :type Integer))
  (if (== OtherActor (`GameplayStatics.GetPlayerCharacter` 0))
    (`KismetSystemLibrary.K2_ClearAndInvalidateTimerHandle` (`self.AuraDamageTimer`))))

(fn `GetIdealRange`
  (returns (AttackRadius :type "Float (double-precision)") (DefendRadius :type "Float (double-precision)") (ChargeRadius :type "Float (double-precision)"))
  (return 200.0 800.0 0.0))

(fn `UserConstructionScript`
  (`parent.UserConstructionScript`))