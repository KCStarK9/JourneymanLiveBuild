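; Melee brute enemy character that punches the player, knocks them back and supplies its own movement speeds and combat ranges.
; PrimaryAttack plays a punch montage whose hit notify box-traces from the hand socket to deal random damage, then signals attack end.
; Pushback box-traces ahead, spawns a shockwave at the player and launches them after a brief delay.
; Charge has a very high speed setting, but its montage code is unwired.
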(event `self.ReceiveTick`
  (params (DeltaSeconds :type "Float (single-precision)"))
  (`parent.ReceiveTick` 0.0))

(event `self.ReceiveBeginPlay`
  (`parent.ReceiveBeginPlay`)
  (bind _asbp_the_gun_panda (cast `/Game/MainBlueprints/Characters/MainCharacter/BP_TheGunPanda` (`GameplayStatics.GetPlayerCharacter` 0)))
  (set `self.As Player` _asbp_the_gun_panda))

(event `/Game/Nick_AI/AI/Logic/BPI_EnemyInterface.PrimaryAttack`
  (params (AttackTarget :type "Actor Object Reference"))
  (bind _returnvalue (`self.GetActorForwardVector`))
  (bind ((`SnowLeopardMeleeDamage_17_F43159D044A5FD7B20663D8D1E5CDFA6` _snowleopardmeleedamage) (`SnowLeopardMeleeDamageMAX_18_12DCEF944C859A18C346BDA4F055D5CC` _snowleopardmeleedamagemax)) (break `/Game/Nick_AI/AI/Logic/Structures/D_EnemyDamages` (`self.DamageStruct`)))
  (bind _returnvalue_2 (`SceneComponent.GetSocketLocation` (`self.Mesh`) "RightHit"))
  ;[1 1 1] Brute Melee Attack
  (`parent.PrimaryAttack` AttackTarget)
  (bind _notifyname (`|PlayMontage` (`self.Mesh`) "/Game/Nick_AI/AI/Enemy_Blueprints/BruteEnemy/Animations/AM_BrutePunch.AM_BrutePunch" 2.0)
    (:`OnCompleted`
      (`/Game/Nick_AI/AI/Logic/BPI_EnemyInterface.AttackEnd` AttackTarget :!label _label)
      (`self.OnAttackEnd`))
    (:`OnInterrupted`
      (goto _label))
    (:`OnNotifyBegin`
      (switch `name` _notifyname
        (:`RightHit`
          (bind (_outhit _returnvalue_3) (`KismetSystemLibrary.BoxTraceSingleForObjects` (+ _returnvalue_2 (* _returnvalue 10.0)) (+ _returnvalue_2 (* _returnvalue 40.0)) (40.0 40.0 20.0) (`self.K2_GetActorRotation`) (`|MakeArray` "ObjectTypeQuery3" :!type "EObjectTypeQuery Enum") false (`|MakeArray` self :!type "Actor Object Reference")))
          (if _returnvalue_3
            (bind _asbp_the_gun_panda (cast `/Game/MainBlueprints/Characters/MainCharacter/BP_TheGunPanda` (`.HitActor` (`GameplayStatics.BreakHitResult` _outhit))))
            (`GameplayStatics.ApplyDamage` _asbp_the_gun_panda (`KismetMathLibrary.RandomFloatInRange` _snowleopardmeleedamage _snowleopardmeleedamagemax))))))))

(event `Pushback`
  (bind _returnvalue (`self.GetActorForwardVector`))
  (bind _boxpushbackspawnpoint (`self.BoxPushbackSpawnPoint`))
  (bind _returnvalue_2 (`SceneComponent.K2_GetComponentLocation` _boxpushbackspawnpoint))
  (bind (_returnvalue_x _returnvalue_y) (`KismetMathLibrary.BreakVector` (* (`self.GetActorForwardVector`) 1000.0)))
  ;[1 1 1] Charge and Knockback
  (bind (_outhit _returnvalue_3) (`KismetSystemLibrary.BoxTraceSingleForObjects` (+ _returnvalue_2 (* _returnvalue 100.0)) (+ _returnvalue_2 (* _returnvalue 200.0)) (20.0 50.0 50.0) (`SceneComponent.K2_GetComponentRotation` _boxpushbackspawnpoint) (`|MakeArray` "ObjectTypeQuery3" :!type "EObjectTypeQuery Enum") false (`|MakeArray` self :!type "Actor Object Reference") "ForDuration"))
  (if _returnvalue_3
    (bind _returnvalue_4 (`NiagaraFunctionLibrary.SpawnSystemAtLocation` "/Game/Nick_AI/VFX/Shockwave/NS_Shockwave.NS_Shockwave" (`self.K2_GetActorLocation` (`self.As Player`)) (`self.K2_GetActorRotation`)))
    (`KismetSystemLibrary.Delay` 0.2)
    (`self.LaunchCharacter` (`self.As Player`) (`KismetMathLibrary.MakeVector` _returnvalue_x _returnvalue_y 2.0) false true)
    (`ActorComponent.Deactivate` _returnvalue_4)))

(fn `GetIdealRange`
  (returns (AttackRadius :type "Float (double-precision)") (DefendRadius :type "Float (double-precision)") (ChargeRadius :type "Float (double-precision)"))
  (return 200.0 450.0 1000.0))

(fn `SetMovementSpeed`
  (params (`Movement Type` :type "/Game/Nick_AI/AI/Logic/Enumerations/E_EnemyMovementSpeed Enum" :default "NewEnumerator0"))
  (returns (`Movement Speed` :type "Float (double-precision)"))
  (bind _output_get (set `CharacterMovementComponent.MaxWalkSpeed` (select `/Game/Nick_AI/AI/Logic/Enumerations/E_EnemyMovementSpeed` `Movement Type` :`NewEnumerator1` 150.0 :`NewEnumerator2` 300.0 :`NewEnumerator3` 600.0 :`NewEnumerator4` 20000.0 :`NewEnumerator7` 100.0) (`self.CharacterMovement`)))
  (return _output_get))

(fn `UserConstructionScript`
  (`parent.UserConstructionScript`))