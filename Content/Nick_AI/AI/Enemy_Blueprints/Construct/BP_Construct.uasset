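; BP_Construct is an AI enemy with a melee attack and a ranged orb/beam attack against the player.
; Melee box-traces on a montage notify to damage BP_TheGunPanda, while ChargeOrb's notify charges a beam from the Shield socket through BPCEnemyAttacks.
; ConstructOrb sends the orb at the player, and each attack signals its end to the AI.
; It also randomly plays hit reactions and supplies its own movement speeds and ideal ranges.
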(event `/Game/Nick_AI/AI/Logic/BPI_EnemyInterface.ChargeOrb`
  (params (`Attack Targer` :type "Actor Object Reference"))
  (`parent.PrimaryAttack` `Attack Targer`)
  (`KismetSystemLibrary.PrintString` "Attack Performed")
  (bind _notifyname (`|PlayMontage` (`self.Mesh`) "/Game/Nick_AI/AI/Enemy_Blueprints/Construct/Animations/Montages/AM_ConstructBlock.AM_ConstructBlock" 0.15)
    (:`OnCompleted`
      (`self.OnAttackEnd` :!label _label)
      (`/Game/Nick_AI/AI/Logic/BPI_EnemyInterface.AttackEnd` `Attack Targer`))
    (:`OnInterrupted`
      (goto _label))
    (:`OnNotifyBegin`
      (switch `name` _notifyname
        (:`ChargeOrb`
          (bind _asai_controller (cast `/Game/Nick_AI/AI/Enemy_Blueprints/AI_Controller` (`AIBlueprintHelperLibrary.GetAIController` self)))
          (bind _attack_target (`/Game/Nick_AI/AI/Enemy_Blueprints/AI_Controller.Attack Target` _asai_controller)
            (:`then`
              (`/Game/Nick_AI/SimpleProjectile/BPC_EnemyAttacks.Charge ConstructBeam` (`self.BPC_EnemyAttacks`) (`SceneComponent.K2_GetComponentToWorld` (`self.Scene`)) _attack_target))
            (:`else`)))))))

(event `/Game/Nick_AI/AI/Logic/BPI_EnemyInterface.ConstructOrb`
  (params (AttackTarget :type "Actor Object Reference"))
  (bind _orb (`/Game/Nick_AI/SimpleProjectile/BPC_EnemyAttacks.Orb` (`self.BPC_EnemyAttacks`)))
  (`parent.ConstructOrb` AttackTarget)
  (set `/Game/Nick_AI/SimpleProjectile/BP_Orb.is spawned?` true _orb)
  (`/Game/Nick_AI/SimpleProjectile/BP_Orb.ChargePlayer` _orb)
  (`KismetSystemLibrary.Delay` 0.2)
  (`self.OnAttackEnd`)
  (`/Game/Nick_AI/AI/Logic/BPI_EnemyInterface.AttackEnd` AttackTarget))

(event `/Game/Nick_AI/AI/Logic/BPI_EnemyInterface.PrimaryAttack`
  (params (AttackTarget :type "Actor Object Reference"))
  (bind _returnvalue (`self.K2_GetActorLocation`))
  (bind _returnvalue_2 (`self.GetActorForwardVector`))
  (bind ((`ConstructMeleeDamage_7_0EF277674F5662DC1E444BA9A6F532A5` _constructmeleedamage) (`ConstructMeleeDamageMAX_8_E9CC069649A30E4781BF41865F81A3F2` _constructmeleedamagemax)) (break `/Game/Nick_AI/AI/Logic/Structures/D_EnemyDamages` (`self.DamageStruct`)))
  (`parent.PrimaryAttack` AttackTarget)
  (bind _notifyname (`|PlayMontage` (`self.Mesh`) "/Game/Nick_AI/AI/Enemy_Blueprints/Construct/Animations/Montages/AM_Construct_Melee.AM_Construct_Melee" 1.5)
    (:`OnCompleted`
      (`self.OnAttackEnd` :!label _label_2)
      (`/Game/Nick_AI/AI/Logic/BPI_EnemyInterface.AttackEnd` AttackTarget))
    (:`OnInterrupted`
      (goto _label_2))
    (:`OnNotifyBegin`
      (switch `name` _notifyname
        (:`Melee`
          (bind (_outhit _returnvalue_3) (`KismetSystemLibrary.BoxTraceSingleForObjects` (+ _returnvalue (* _returnvalue_2 100.0)) (+ _returnvalue (* _returnvalue_2 100.0)) (30.0 50.0 20.0) (`self.K2_GetActorRotation`) (`|MakeArray` "ObjectTypeQuery3" :!type "EObjectTypeQuery Enum") false (`|MakeArray` self :!type "Actor Object Reference") "None" true (struct :`R` 1.0 :`A` 1.0) (struct :`R` 0.064528 :`G` 0.291361 :`B` 1.0 :`A` 1.0)))
          (if _returnvalue_3
            (bind _asbp_the_gun_panda (cast `/Game/MainBlueprints/Characters/MainCharacter/BP_TheGunPanda` (`.HitActor` (`GameplayStatics.BreakHitResult` _outhit))))
            (`GameplayStatics.ApplyDamage` _asbp_the_gun_panda (`KismetMathLibrary.RandomFloatInRange` _constructmeleedamage _constructmeleedamagemax))))))))

(event `self.ReceiveHit`
  (params (MyComp :type "PrimitiveComponent Object Reference") (Other :type "Actor Object Reference") (OtherComp :type "PrimitiveComponent Object Reference") (bSelfMoved :type Boolean) (HitLocation :type "Vector Structure") (HitNormal :type "Vector Structure") (NormalImpulse :type "Vector Structure") (Hit :type "HitResult Structure (by ref)"))
  (if (`KismetMathLibrary.RandomBool`)
    (`|PlayMontage` (`self.Mesh`) "/Game/Nick_AI/AI/Enemy_Blueprints/Construct/Animations/Montages/AM_ConstructHIT.AM_ConstructHIT")))

(fn `GetIdealRange`
  (returns (AttackRadius :type "Float (double-precision)") (DefendRadius :type "Float (double-precision)") (ChargeRadius :type "Float (double-precision)"))
  (return 150.0 300.0 800.0))

(fn `SetMovementSpeed`
  (params (`Movement Type` :type "/Game/Nick_AI/AI/Logic/Enumerations/E_EnemyMovementSpeed Enum" :default "NewEnumerator0"))
  (returns (`Movement Speed` :type "Float (double-precision)"))
  (set `CharacterMovementComponent.MaxWalkSpeed` (select `/Game/Nick_AI/AI/Logic/Enumerations/E_EnemyMovementSpeed` `Movement Type` :`NewEnumerator1` 250.0 :`NewEnumerator2` 300.0) (`self.CharacterMovement`))
  (return 0.0))

(fn `UserConstructionScript`
  (`parent.UserConstructionScript`)
  (`SceneComponent.K2_AttachToComponent` (`self.Scene`) (`self.Mesh`) "Shield" "SnapToTarget" "SnapToTarget" "SnapToTarget" true))