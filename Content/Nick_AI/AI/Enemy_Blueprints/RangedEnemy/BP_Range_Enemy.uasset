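; BP_Range_Enemy is a gun-carrying ranged AI enemy that overrides its parent's attack, movement speed and ideal range.
; PrimaryAttack calls Warning and plays a montage whose notifies spawn a muzzle flash or, given a valid AI target, warn the player, play a shot sound and fire through BPCEnemyAttacks.
; Montage completion or interruption ends the attack.
; Construction snaps the gun to a mesh socket.
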(event `self.PrimaryAttack`
  (params (AttackTarget :type "Actor Object Reference"))
  (bind _scene (`self.Scene`))
  (bind _returnvalue (`SceneComponent.K2_GetComponentLocation` _scene))
  (`parent.PrimaryAttack` AttackTarget)
  (`KismetSystemLibrary.PrintString` "Attack Performed")
  (`|ExecutionSequence`
    (:`then_0`
      (bind _notifyname (`|PlayMontage` (`self.Mesh`) (`self.Montage to Play_0`) 2.0)
        (:`OnCompleted`
          (`self.OnAttackEnd` :!label _label)
          (`self.AttackEnd` AttackTarget))
        (:`OnInterrupted`
          (goto _label))
        (:`OnNotifyBegin`
          (switch `name` _notifyname
            (:`Fire`
              (bind _asai_controller (cast `/Game/Nick_AI/AI/Enemy_Blueprints/AI_Controller` (`AIBlueprintHelperLibrary.GetAIController` self)))
              (bind _attack_target (`/Game/Nick_AI/AI/Enemy_Blueprints/AI_Controller.Attack Target` _asai_controller)
                (:`then`
                  (bind _asbp_the_gun_panda (cast `/Game/MainBlueprints/Characters/MainCharacter/BP_TheGunPanda` (`GameplayStatics.GetPlayerCharacter` 0)))
                  (`/Game/MainBlueprints/Characters/MainCharacter/BP_TheGunPanda.Warning` _asbp_the_gun_panda)
                  (`GameplayStatics.PlaySoundAtLocation` "/Game/MainBlueprints/SoundAssets/SoundCues/Shot_2_Cue.Shot_2_Cue" _returnvalue (struct) 1.0 1.0 0.0 null null null null)
                  (`/Game/Nick_AI/SimpleProjectile/BPC_EnemyAttacks.RangedEnemyAttack` (`self.BPC_EnemyAttacks`) (`SceneComponent.K2_GetComponentToWorld` _scene) _attack_target))
                (:`else`)))
            (:`Flash`
              (`NiagaraFunctionLibrary.SpawnSystemAtLocation` "/Game/Nick_AI/VFX/BulletTrail/NS_Muzzle.NS_Muzzle" _returnvalue (`SceneComponent.K2_GetComponentRotation` _scene)))))))
    (:`then_1`
      (`self.Warning`))))

(fn `GetIdealRange`
  (returns (AttackRadius :type "Float (double-precision)") (DefendRadius :type "Float (double-precision)") (ChargeRadius :type "Float (double-precision)"))
  (return 600.0 600.0 0.0))

(fn `SetMovementSpeed`
  (params (`Movement Type` :type "/Game/Nick_AI/AI/Logic/Enumerations/E_EnemyMovementSpeed Enum" :default "NewEnumerator0"))
  (returns (`Movement Speed` :type "Float (double-precision)"))
  (bind _output_get (set `CharacterMovementComponent.MaxWalkSpeed` (select `/Game/Nick_AI/AI/Logic/Enumerations/E_EnemyMovementSpeed` `Movement Type` :`NewEnumerator1` 200.0 :`NewEnumerator2` 300.0 :`NewEnumerator3` 500.0) (`self.CharacterMovement`)))
  (return _output_get))

(fn `UserConstructionScript`
  (`parent.UserConstructionScript`)
  (`SceneComponent.K2_AttachToComponent` (`self.Gun`) (`self.Mesh`) "Gun_Socket" "SnapToTarget" "SnapToTarget" "SnapToTarget" true))