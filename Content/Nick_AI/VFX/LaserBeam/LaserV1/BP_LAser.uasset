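; BP_LAser is a laser beam actor that slowly turns toward its Target and damages what it hits.
; Each tick it extends its range up to a cap, traces, updates beam and impact effects and applies small random damage.
; A second trace positions a radial strain field for physics destruction.
; On a hit, range snaps to the hit distance and a delayed self-destroy starts.
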(event `self.ReceiveBeginPlay`
  (`|ExecutionSequence`
    (:`then_0`
      (`FXSystemComponent.SetColorParameter` (`self.Laser`) "Colour" (struct :`R` 0.048577 :`G` 0.811559 :`B` 1.1 :`A` 1.0))
      (`FXSystemComponent.SetColorParameter` (`self.Impact`) "Colour" (struct :`G` 0.704294 :`B` 1.1 :`A` 1.0))
      (bind _asbp_the_gun_panda (cast `/Game/MainBlueprints/Characters/MainCharacter/BP_TheGunPanda` (`GameplayStatics.GetPlayerCharacter` 0)))
      (set `self.As BP The Gun Panda` _asbp_the_gun_panda))
    (:`then_1`
      (`PrimitiveComponent.IgnoreActorWhenMoving` (`self.Laser`) (`self.GetOwner`) true))))

(event `self.ReceiveTick`
  (params (DeltaSeconds :type "Float (single-precision)"))
  (bind _returnvalue (`self.K2_GetActorLocation`))
  (bind _returnvalue_2 (`self.K2_GetActorLocation`))
  (bind _returnvalue_3 (+ _returnvalue (* (`self.GetActorForwardVector`) (`self.LaserDistance`))))
  (`self.K2_SetActorRotation` (`KismetMathLibrary.RInterpTo` (`self.K2_GetActorRotation`) (`KismetMathLibrary.FindLookAtRotation` (`self.K2_GetActorLocation`) (`self.K2_GetActorLocation` (`self.Target`))) (`GameplayStatics.GetWorldDeltaSeconds`) 1.0))
  (`|ExecutionSequence`
    (:`then_0`
      (bind (_outhit _returnvalue_4) (`KismetSystemLibrary.LineTraceSingleForObjects` _returnvalue _returnvalue_3 (`|MakeArray` "ObjectTypeQuery1" "ObjectTypeQuery2" "ObjectTypeQuery3" "ObjectTypeQuery6" "ObjectTypeQuery7" :!type "EObjectTypeQuery Enum") false (`|MakeArray` self (`self.GetInstigator`) (`self.Instigator`) :!type "Actor Object Reference")))
      (`|ExecutionSequence`
        (:`then_0`
          (bind (_bblockinghit _binitialoverlap _time _distance _location _impactpoint _normal _impactnormal _physmat _hitactor) (`GameplayStatics.BreakHitResult` _outhit))
          (`FXSystemComponent.SetVectorParameter` (`self.Laser`) "EndLocation" (select `bool` _returnvalue_4 :`false` _returnvalue_3 :`true` _location))
          (`|ExecutionSequence`
            (:`then_0`
              (`SceneComponent.SetVisibility` (`self.Impact`) _returnvalue_4 false)
              (`SceneComponent.K2_SetWorldLocation` (`self.Impact`) _impactpoint false false)
              (if _returnvalue_4
                (set `self.LaserDistance` (`KismetMathLibrary.VSize` (- _location (`self.K2_GetActorLocation`))))
                (`KismetSystemLibrary.Delay` 3.0)
                (`self.K2_DestroyActor`)))
            (:`then_1`
              (`GameplayStatics.ApplyDamage` _hitactor (`KismetMathLibrary.RandomFloatInRange` 0.1 0.3) null self))))))
    (:`then_1`
      (if (< (`self.LaserDistance`) 10000.0)
        (set `self.LaserDistance` (+ (`self.LaserDistance`) (* DeltaSeconds 2500.0)))))
    (:`then_2`
      (bind _outhit_2 (`KismetSystemLibrary.LineTraceSingle` _returnvalue_2 (+ _returnvalue_2 (* (`self.GetActorForwardVector`) (`self.LaserDistance`))) "TraceTypeQuery1" false (`|MakeArray` self (`self.Target`) :!type "Actor Object Reference") "None" true (struct :`G` 0.717875 :`B` 1.0 :`A` 1.0)))
      (`FieldSystemComponent.ApplyPhysicsField` (`self.FieldSystem`) true "Field_ExternalClusterStrain" null (`RadialFalloff.SetRadialFalloff` (`self.RadialFalloff`) 500000.0 0.0 1.0 0.0 250.0 (`.ImpactPoint` (`GameplayStatics.BreakHitResult` _outhit_2)) "Field_FallOff_None")))))

(fn `UserConstructionScript`)