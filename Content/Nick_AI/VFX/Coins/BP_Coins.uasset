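; BP_Coins is a coin pickup that gets pulled toward the player and vanishes on contact.
; When the player character enters PullBox, the MoveToChar timeline interpolates the coin toward the player's current location each update, adding the timeline track's value as an offset.
; When CoinMesh overlaps the player, it plays the BagOcoins sound in 2D and destroys the actor, without updating any score or currency.
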(event `self.PullBox.OnComponentBeginOverlap`
  (params (OverlappedComponent :type "PrimitiveComponent Object Reference") (OtherActor :type "Actor Object Reference") (OtherComp :type "PrimitiveComponent Object Reference") (OtherBodyIndex :type Integer) (bFromSweep :type Boolean) (SweepResult :type "HitResult Structure (by ref)"))
  (if (== OtherActor (`GameplayStatics.GetPlayerCharacter` 0))
    (bind (_direction _newtrack_0) (`Timeline|Move to char` :!via `PlayFromStart`)
      (:`Update`
        (`self.K2_SetActorLocation` (+ _newtrack_0 (`KismetMathLibrary.VInterpTo` (`self.K2_GetActorLocation`) (`self.K2_GetActorLocation` (`GameplayStatics.GetPlayerCharacter` 0)) (`GameplayStatics.GetWorldDeltaSeconds`) 10.0)))))))

(event `self.CoinMesh.OnComponentBeginOverlap`
  (params (OverlappedComponent :type "PrimitiveComponent Object Reference") (OtherActor :type "Actor Object Reference") (OtherComp :type "PrimitiveComponent Object Reference") (OtherBodyIndex :type Integer) (bFromSweep :type Boolean) (SweepResult :type "HitResult Structure (by ref)"))
  (if (== OtherActor (`GameplayStatics.GetPlayerCharacter` 0))
    (`GameplayStatics.PlaySound2D` "/Game/Nick_AI/VFX/Coins/BagOcoins.BagOcoins" 1.0 1.0 0.0 null null)
    (`self.K2_DestroyActor`)))

(fn `UserConstructionScript`)