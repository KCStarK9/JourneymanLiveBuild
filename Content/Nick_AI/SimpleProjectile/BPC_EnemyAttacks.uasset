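; Enemy attack component that spawns targeted projectiles, a boss fist, a boss laser and construct orbs.
; Projectile and fist impacts apply random damage from DamageStruct ranges and, like orb hits, fire OnAttackEnded; the laser is only spawned and stored.
; ChargeConstructBeam staggers three orbs that charge the player after a delay, sharing one Orb reference.
; Orb hits show a brief shockwave and temporarily slow the Gun Panda player, with no damage amount set.
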(event `self.ReceiveBeginPlay`
  (bind _asbp_the_gun_panda (cast `/Game/MainBlueprints/Characters/MainCharacter/BP_TheGunPanda` (`GameplayStatics.GetPlayerCharacter` 0)))
  (set `self.As BP The Gun Panda` _asbp_the_gun_panda))

(event `RangedEnemyAttack`
  (params (SpawnTransform :type "Transform Structure") (Target :type "Actor Object Reference"))
  (bind _returnvalue (`|SpawnActorFromClass` "/Game/Nick_AI/SimpleProjectile/BP_Tier1_Projectile.BP_Tier1_Projectile_C" SpawnTransform "Undefined" "MultiplyWithRoot" (`self.GetOwner`) Target 2000.0 0.0 null))
  (add `/Game/Nick_AI/SimpleProjectile/BP_ProjectileBase.OnProjectileImpact` _returnvalue (delegate `OnImpact`)))

(event `OnImpact`
  (params (OtherActor :type "Actor Object Reference") (`Hit Result` :type "HitResult Structure"))
  (bind ((`PineMartinDamage_11_B879CF5B430648D2913CDD8EFD61357C` _pinemartindamage) (`PineMartinDamageMAX_12_D51445D34D3EEE45679BA6A4538E5C3C` _pinemartindamagemax)) (break `/Game/Nick_AI/AI/Logic/Structures/D_EnemyDamages` (`self.DamageStruct`)))
  (`GameplayStatics.ApplyDamage` (`.HitActor` (`GameplayStatics.BreakHitResult` `Hit Result`)) (`KismetMathLibrary.RandomFloatInRange` _pinemartindamage _pinemartindamagemax))
  (`self.OnAttackEnded`))

(event `LaunchFist`
  (params (Target :type "Actor Object Reference") (SpawnTransform :type "Transform Structure"))
  (bind _returnvalue (`|SpawnActorFromClass` "/Game/Nick_AI/SimpleProjectile/BP_RightFist.BP_RightFist_C" SpawnTransform "Undefined" "MultiplyWithRoot" (`self.GetOwner`) Target 3500.0 0.0 null))
  (add `/Game/Nick_AI/SimpleProjectile/BP_ProjectileBase.OnProjectileImpact` _returnvalue (delegate `FistImpact`)))

(event `FistImpact`
  (params (OtherActor :type "Actor Object Reference") (`Hit Result` :type "HitResult Structure"))
  (bind ((`BossFistProjectileDamage_23_74D16C424FBD023F9942C2BC07E78CAA` _bossfistprojectiledamage) (`BossFistProjectileDamageMAX_24_3C7F62B7428B09E706FC94BD8C235433` _bossfistprojectiledamagemax)) (break `/Game/Nick_AI/AI/Logic/Structures/D_EnemyDamages` (`self.DamageStruct`)))
  (`GameplayStatics.ApplyDamage` OtherActor (`KismetMathLibrary.RandomFloatInRange` _bossfistprojectiledamage _bossfistprojectiledamagemax))
  (`self.OnAttackEnded`))

(event `FireBossLaser`
  (params (SpawnTransform :type "Transform Structure") (Target :type "Actor Object Reference"))
  (bind _returnvalue (`self.GetOwner`))
  (bind _returnvalue_2 (`|SpawnActorFromClass` "/Game/Nick_AI/VFX/LaserBeam/LaserV1/BP_LAser.BP_LAser_C" SpawnTransform "Undefined" "MultiplyWithRoot" _returnvalue Target (`Actor.Instigator` _returnvalue)))
  (set `self.LaserREF` _returnvalue_2))

(event `Charge ConstructBeam`
  (params (SpawnTransform :type "Transform Structure") (Target :type "Actor Object Reference"))
  (`|ExecutionSequence`
    (:`then_0`
      (bind _returnvalue (`|SpawnActorFromClass` "/Game/Nick_AI/SimpleProjectile/BP_Orb.BP_Orb_C" SpawnTransform "Undefined" "MultiplyWithRoot" (`self.GetOwner`) Target 1000.0 0.0 null))
      (`/Engine/EditorBlueprintResources/StandardMacros.IsValid` _returnvalue
        (:`Is Valid`
          (bind _output_get (set `self.Orb` _returnvalue))
          (add `/Game/Nick_AI/SimpleProjectile/BP_ProjectileBase.OnProjectileImpact` _output_get (delegate `onProjectileHit`))
          (`KismetSystemLibrary.Delay` 0.6)
          (`/Game/Nick_AI/SimpleProjectile/BP_Orb.ChargePlayer` (`self.Orb`)))))
    (:`then_1`
      (`KismetSystemLibrary.Delay` 1.1)
      (bind _returnvalue_2 (`|SpawnActorFromClass` "/Game/Nick_AI/SimpleProjectile/BP_Orb.BP_Orb_C" SpawnTransform "Undefined" "MultiplyWithRoot" (`self.GetOwner`) Target 1000.0 0.0 null))
      (`/Engine/EditorBlueprintResources/StandardMacros.IsValid` _returnvalue_2
        (:`Is Valid`
          (bind _output_get_2 (set `self.Orb` _returnvalue_2))
          (add `/Game/Nick_AI/SimpleProjectile/BP_ProjectileBase.OnProjectileImpact` _output_get_2 (delegate `onhit2`))
          (`KismetSystemLibrary.Delay` 0.6)
          (`/Game/Nick_AI/SimpleProjectile/BP_Orb.ChargePlayer` (`self.Orb`)))))
    (:`then_2`
      (`KismetSystemLibrary.Delay` 2.3)
      (bind _returnvalue_3 (`|SpawnActorFromClass` "/Game/Nick_AI/SimpleProjectile/BP_Orb.BP_Orb_C" SpawnTransform "Undefined" "MultiplyWithRoot" (`self.GetOwner`) Target 1000.0 0.0 null))
      (`/Engine/EditorBlueprintResources/StandardMacros.IsValid` _returnvalue_3
        (:`Is Valid`
          (bind _output_get_3 (set `self.Orb` _returnvalue_3))
          (add `/Game/Nick_AI/SimpleProjectile/BP_ProjectileBase.OnProjectileImpact` _output_get_3 (delegate `on hit 3`))
          (`KismetSystemLibrary.Delay` 0.6)
          (`/Game/Nick_AI/SimpleProjectile/BP_Orb.ChargePlayer` (`self.Orb`)))))))

(event `onProjectileHit`
  (params (OtherActor :type "Actor Object Reference") (`Hit Result` :type "HitResult Structure"))
  (bind (_bblockinghit _binitialoverlap _time _distance _location _impactpoint _normal _impactnormal _physmat _hitactor) (`GameplayStatics.BreakHitResult` `Hit Result`))
  (bind _orb (`self.Orb`))
  (bind _charactermovement (`Character.CharacterMovement` (`self.As BP The Gun Panda`)))
  (`GameplayStatics.ApplyDamage` OtherActor)
  (`self.OnAttackEnded`)
  (bind _returnvalue (`NiagaraFunctionLibrary.SpawnSystemAtLocation` "/Game/Nick_AI/VFX/Shockwave/NS_ShockwaveYellow.NS_ShockwaveYellow" _location))
  (`KismetSystemLibrary.Delay` 0.2)
  (`self.Deactivate` _returnvalue)
  (`/Engine/EditorBlueprintResources/StandardMacros.IsValid` _orb
    (:`Is Valid`
      (set `/Game/Nick_AI/SimpleProjectile/BP_Orb.is spawned?` false _orb)
      (if (== _hitactor (`self.As BP The Gun Panda`))
        (set `CharacterMovementComponent.MaxWalkSpeed` 200.0 _charactermovement)
        (`KismetSystemLibrary.Delay` 2.0)
        (set `CharacterMovementComponent.MaxWalkSpeed` 600.0 _charactermovement)))))

(event `onhit2`
  (params (OtherActor :type "Actor Object Reference") (`Hit Result` :type "HitResult Structure"))
  (bind (_bblockinghit _binitialoverlap _time _distance _location _impactpoint _normal _impactnormal _physmat _hitactor) (`GameplayStatics.BreakHitResult` `Hit Result`))
  (bind _orb (`self.Orb`))
  (bind _charactermovement (`Character.CharacterMovement` (`self.As BP The Gun Panda`)))
  (`GameplayStatics.ApplyDamage` OtherActor)
  (`self.OnAttackEnded`)
  (bind _returnvalue (`NiagaraFunctionLibrary.SpawnSystemAtLocation` "/Game/Nick_AI/VFX/Shockwave/NS_ShockwaveYellow.NS_ShockwaveYellow" _location))
  (`KismetSystemLibrary.Delay` 0.2)
  (`self.Deactivate` _returnvalue)
  (`/Engine/EditorBlueprintResources/StandardMacros.IsValid` _orb
    (:`Is Valid`
      (set `/Game/Nick_AI/SimpleProjectile/BP_Orb.is spawned?` false _orb)
      (if (== _hitactor (`self.As BP The Gun Panda`))
        (set `CharacterMovementComponent.MaxWalkSpeed` 200.0 _charactermovement)
        (`KismetSystemLibrary.Delay` 2.0)
        (set `CharacterMovementComponent.MaxWalkSpeed` 600.0 _charactermovement)))))

(event `on hit 3`
  (params (OtherActor :type "Actor Object Reference") (`Hit Result` :type "HitResult Structure"))
  (bind (_bblockinghit _binitialoverlap _time _distance _location _impactpoint _normal _impactnormal _physmat _hitactor) (`GameplayStatics.BreakHitResult` `Hit Result`))
  (bind _orb (`self.Orb`))
  (bind _charactermovement (`Character.CharacterMovement` (`self.As BP The Gun Panda`)))
  (`GameplayStatics.ApplyDamage` OtherActor)
  (`self.OnAttackEnded`)
  (bind _returnvalue (`NiagaraFunctionLibrary.SpawnSystemAtLocation` "/Game/Nick_AI/VFX/Shockwave/NS_ShockwaveYellow.NS_ShockwaveYellow" _location))
  (`KismetSystemLibrary.Delay` 0.2)
  (`self.Deactivate` _returnvalue)
  (`/Engine/EditorBlueprintResources/StandardMacros.IsValid` _orb
    (:`Is Valid`
      (set `/Game/Nick_AI/SimpleProjectile/BP_Orb.is spawned?` false _orb)
      (if (== _hitactor (`self.As BP The Gun Panda`))
        (set `CharacterMovementComponent.MaxWalkSpeed` 200.0 _charactermovement)
        (`KismetSystemLibrary.Delay` 2.0)
        (set `CharacterMovementComponent.MaxWalkSpeed` 600.0 _charactermovement)))))

(fn `SpawnOrb`
  (params (SpawnTransform :type "Transform Structure") (Target :type "Actor Object Reference"))
  (returns (ReturnValue :type "NiagaraComponent Object Reference"))
  (bind _returnvalue (`|SpawnActorFromClass` "/Game/Nick_AI/SimpleProjectile/BP_Orb.BP_Orb_C" SpawnTransform "Undefined" "MultiplyWithRoot" (`self.GetOwner`) Target 1000.0 0.0 null))
  (set `self.Orb` _returnvalue))