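; BP_Orb is an AI projectile orb that grows in on spawn and can be launched at the player.
; On BeginPlay it caches the player's BP_TheGunPanda and plays a one-shot timeline that scales the Orb effect's size, emissive, inner-orb and distortion parameters.
; While IsSpawned is true, Tick calls RotateToTarget, and the ChargePlayer event activates ProjectileMovement.
; An inline yaw-only look-at rotation toward the player is left unconnected.
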(event `self.ReceiveBeginPlay`
  (`parent.ReceiveBeginPlay`)
  (`|ExecutionSequence`
    (:`then_0`
      (bind _asbp_the_gun_panda (cast `/Game/MainBlueprints/Characters/MainCharacter/BP_TheGunPanda` (`GameplayStatics.GetPlayerCharacter` 0)))
      (set `self.As BP The Gun Panda` _asbp_the_gun_panda))
    (:`then_1`
      (`/Engine/EditorBlueprintResources/StandardMacros.DoOnce` false
        (:`Completed`
          (bind (_direction _orbgrowth) (`Timeline|Timeline` :!via `PlayFromStart`)
            (:`Update`
              (`FXSystemComponent.SetFloatParameter` (`self.Orb`) "OrbSize" (`KismetMathLibrary.Lerp` 0.0 0.5 _orbgrowth))
              (`FXSystemComponent.SetFloatParameter` (`self.Orb`) "EmissiveSize" (`KismetMathLibrary.Lerp` 0.0 1.0 _orbgrowth))
              (`FXSystemComponent.SetFloatParameter` (`self.Orb`) "InnerOrb" (`KismetMathLibrary.Lerp` 0.0 1.0 _orbgrowth))
              (`FXSystemComponent.SetFloatParameter` (`self.Orb`) "Distortion Size" (`KismetMathLibrary.Lerp` 0.0 0.5 _orbgrowth)))))))))

(event `self.ReceiveTick`
  (params (DeltaSeconds :type "Float (single-precision)"))
  (if (`self.is spawned?`)
    (`self.RotateToTarget`)))

(event `ChargePlayer`
  (`ActorComponent.Activate` (`self.ProjectileMovement`) false))

(fn `UserConstructionScript`
  (`parent.UserConstructionScript`))