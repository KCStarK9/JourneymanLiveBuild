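; BP_RightFist is a right-fist actor that fractures Chaos destructible geometry in front of it.
; Every Tick it line-traces forward on the Visibility channel from its location.
; The impact point centers a radial falloff node, which the Field System applies as a strong, non-attenuated external cluster strain.
; The trace result is not checked, so the field is applied every frame even without a hit.
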(event `self.ReceiveTick`
  (params (DeltaSeconds :type "Float (single-precision)"))
  (bind _returnvalue (`self.K2_GetActorLocation`))
  (bind _outhit (`KismetSystemLibrary.LineTraceSingle` _returnvalue (+ _returnvalue (* (`self.GetActorForwardVector`) 1000.0)) "TraceTypeQuery1" false (`|MakeArray` self null :!type "Actor Object Reference") "None" true (struct :`G` 0.717875 :`B` 1.0 :`A` 1.0)))
  (`FieldSystemComponent.ApplyPhysicsField` (`self.FieldSystem`) true "Field_ExternalClusterStrain" null (`RadialFalloff.SetRadialFalloff` (`self.RadialFalloff`) 500000.0 0.0 1.0 0.0 250.0 (`.ImpactPoint` (`GameplayStatics.BreakHitResult` _outhit)) "Field_FallOff_None")))

(fn `UserConstructionScript`
  (`parent.UserConstructionScript`))