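; Interactable dungeon cell door that swings open from one side only and has no closing logic.
; TryInteract calls the parent, then uses a dot product with the actor's forward vector to accept only characters on the front side.
; A looping timer, guarded against restarts, drives stepped yaw rotation of the door mesh instead of Tick.
; At the clamped open angle, the door is flagged open and the timer is invalidated.
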(event `OpenTheDoorUpdate`
  (bind _output_get (set `self.cur_angle` (`KismetMathLibrary.FMax` (+ (`self.cur_angle`) (* 0.1 -100.0)) -90.0)))
  (`SceneComponent.K2_SetRelativeRotation` (`self.SM_Cell_Door`) (`KismetMathLibrary.MakeRotator` 0.0 0.0 _output_get) false false)
  (if (== (`self.cur_angle`) -90.0)
    (set `self.is_open` true)
    (`KismetSystemLibrary.K2_InvalidateTimerHandle` (`self.update_timer`))))

(fn `TryInteract`
  (params (target_character :type "Character Object Reference"))
  (`parent.TryInteract` target_character)
  (if (not (`self.is_open`))
    (if (> (`KismetMathLibrary.Dot_VectorVector` (`KismetMathLibrary.Normal` (- (`self.K2_GetActorLocation` target_character) (`self.K2_GetActorLocation`))) (`self.GetActorForwardVector`)) 0.0)
      (if (not (`KismetSystemLibrary.K2_IsValidTimerHandle` (`self.update_timer`)))
        (bind _returnvalue (`KismetSystemLibrary.K2_SetTimerDelegate` (`|CreateDelegate` :!event `OpenTheDoorUpdate`) 0.1 true))
        (set `self.update_timer` _returnvalue)))))

(fn `UserConstructionScript`
  (`parent.UserConstructionScript`))