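; BP_Door_boosroom_door_1 is a boss room door in the dungeon blockout that slides down out of the way when opened.
; Calling OpenDoor sets a flag and enables ticking.
; Tick eases the door mesh's relative Z toward a fixed lowered position with FInterpTo, then disables its own tick once it reaches that position.
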(event `self.ReceiveTick`
  (params (DeltaSeconds :type "Float (single-precision)"))
  (if (`self.should_open`)
    (bind _output_get (set `self.cur_z` (`KismetMathLibrary.FInterpTo` (`self.cur_z`) -1200.0 DeltaSeconds 5.0)))
    (`SceneComponent.K2_SetRelativeLocation` (`self.door_mesh`) (`KismetMathLibrary.MakeVector` 0.0 0.0 _output_get) false false)
    (if (== (`self.cur_z`) -1200.0)
      (`self.SetActorTickEnabled` false))))

(fn `OpenDoor`
  (set `self.should_open` true)
  (`self.SetActorTickEnabled` true))

(fn `UserConstructionScript`)