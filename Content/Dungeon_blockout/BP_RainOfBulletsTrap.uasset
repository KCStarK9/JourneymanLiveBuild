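; Dungeon trap actor that rains BP_TrapBullet actors while the player pawn is inside its Box.
; Box overlap events store and clear the player pawn reference, which gates a Tick-driven random Delay that paces SpawnBullet.
; SpawnBullet picks a random point on the box's top plane from its unscaled extent and converts it to world space through the actor transform.
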(event `self.ReceiveBeginPlay`)

(event `self.ReceiveTick`
  (params (DeltaSeconds :type "Float (single-precision)"))
  (`self.player_pawn`
    (:`then`
      (`KismetSystemLibrary.Delay` (`KismetMathLibrary.RandomFloatInRange` 0.05 0.5))
      (`self.SpawnBullet`))
    (:`else`)))

(event `self.Box.OnComponentBeginOverlap`
  (params (OverlappedComponent :type "PrimitiveComponent Object Reference") (OtherActor :type "Actor Object Reference") (OtherComp :type "PrimitiveComponent Object Reference") (OtherBodyIndex :type Integer) (bFromSweep :type Boolean) (SweepResult :type "HitResult Structure (by ref)"))
  ;[1 1 1] When the player enters the box, the rain of bullets is generated.
  (if (== OtherActor (`GameplayStatics.GetPlayerPawn` 0))
    (bind _aspawn (cast `Pawn` OtherActor)
      (:`then`
        (set `self.player_pawn` _aspawn))
      (:`CastFailed`
        (`KismetSystemLibrary.PrintString` "Hello")))))

(event `self.Box.OnComponentEndOverlap`
  (params (OverlappedComponent :type "PrimitiveComponent Object Reference") (OtherActor :type "Actor Object Reference") (OtherComp :type "PrimitiveComponent Object Reference") (OtherBodyIndex :type Integer))
  ;[1 1 1] When the player enters the box, the rain of bullets is generated.
  (if (== OtherActor (`GameplayStatics.GetPlayerPawn` 0))
    (set `self.player_pawn` null)))

(fn `SpawnBullet`
  (locals (spawn_location :type "Vector Structure"))
  (bind _x (.x (`BoxComponent.BoxExtent` (`self.Box`))))
  (bind _y (.y (`BoxComponent.BoxExtent` (`self.Box`))))
  ;[1 1 1] This is the spawning point location, the local space location of the actor
  (bind _output_get (set `local.spawn_location` (`KismetMathLibrary.MakeVector` (`KismetMathLibrary.RandomFloatInRange` (* _x -1.0) _x) (`KismetMathLibrary.RandomFloatInRange` (* _y -1.0) _y) (.z (`BoxComponent.BoxExtent` (`self.Box`))))))
  (`|SpawnActorFromClass` "/Game/Dungeon_blockout/BP_TrapBullet.BP_TrapBullet_C" (`KismetMathLibrary.MakeTransform` (`KismetMathLibrary.TransformLocation` (`self.GetTransform`) _output_get)) "Undefined" "MultiplyWithRoot" null null))

(fn `UserConstructionScript`)