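; BP_key1 is a key pickup in the dungeon blockout that sets IsKey01Pickup on the BP_TheGunPanda player.
; Tick runs through a short Delay, then compares the player pawn's distance to the Cube component against PickupRadius instead of using overlap events.
; Within range, a successful cast sets the flag, destroys the actor and prints a debug message.
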(event `self.ReceiveBeginPlay`)

(event `self.ReceiveTick`
  (params (DeltaSeconds :type "Float (single-precision)"))
  (bind _returnvalue (`GameplayStatics.GetPlayerPawn` 0))
  (`KismetSystemLibrary.Delay` 0.3)
  (`/Engine/EditorBlueprintResources/StandardMacros.IsValid` _returnvalue
    (:`Is Valid`
      (if (<= (`KismetMathLibrary.Vector_Distance` (`self.K2_GetActorLocation` _returnvalue) (`SceneComponent.K2_GetComponentLocation` (`self.Cube`))) (`self.pickup_radius`))
        (bind _asbp_the_gun_panda (cast `/Game/MainBlueprints/Characters/MainCharacter/BP_TheGunPanda` _returnvalue)
          (:`then`
            (set `/Game/MainBlueprints/Characters/MainCharacter/BP_TheGunPanda.is_key01_pickup` true _asbp_the_gun_panda)
            (`self.K2_DestroyActor`)
            (`KismetSystemLibrary.PrintString` "Pickup" true true (struct :`R` 1.0 :`G` 0.063993 :`A` 1.0) 10.0))
          (:`CastFailed`
            (`KismetSystemLibrary.PrintString` "Hello")))))))

(fn `UserConstructionScript`)