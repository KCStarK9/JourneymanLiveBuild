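; BP_pillar3 is a dungeon blockout pillar that gets knocked away when kicked.
; OnKick turns on physics simulation for the SMPillar02 mesh and applies a large fixed-strength impulse pointing away from the kicking character.
; The impulse direction is flattened to the horizontal plane and normalized, so the kicker's height and distance do not affect the push.
; The event graph is empty and the construction script only calls its parent.
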(fn `OnKick`
  (params (target_character :type "Character Object Reference"))
  (bind _sm_pillar02 (`self.SM_Pillar02`))
  (`PrimitiveComponent.SetSimulatePhysics` _sm_pillar02 true)
  (`PrimitiveComponent.AddImpulse` _sm_pillar02 (* (`KismetMathLibrary.Normal` (`KismetMathLibrary.MakeVector` (.x (- (`self.K2_GetActorLocation`) (`self.K2_GetActorLocation` target_character))) (.y (- (`self.K2_GetActorLocation`) (`self.K2_GetActorLocation` target_character))))) 80000.0) "None" false))

(fn `UserConstructionScript`
  (`parent.UserConstructionScript`))