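; BP_BestHUD manages the game's screens: boot-up, main menu, gameplay HUD and inventory.
; BootUp plays a timed intro until the game instance flags it done, then shows the main menu.
; LevelBegin creates the gameplay HUD, sets game-only input and caches the GunPanda player.
; InventoryControl toggles a freshly created inventory with keyboard focus, syncing guns to the HUD on close, while CycleGuns forwards weapon switches to the HUD.
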(event `BootUp`
  (bind _asbp_best_game_instance (cast `/Game/MainBlueprints/BP_BestGameInstance` (`GameplayStatics.GetGameInstance`)))
  (if (not (`/Game/MainBlueprints/BP_BestGameInstance.BootUpDone` _asbp_best_game_instance))
    (bind _returnvalue (`|CreateWidget` "/Game/MainBlueprints/Widgets/W_BootUp.W_BootUp_C"))
    (`UserWidget.AddToViewport` _returnvalue 0)
    (`/Game/MainBlueprints/Widgets/W_BootUp.Launch` _returnvalue)
    (`KismetSystemLibrary.Delay` 12.5)
    (set `/Game/MainBlueprints/BP_BestGameInstance.BootUpDone` true _asbp_best_game_instance))
  (bind _returnvalue_2 (`|CreateWidget` "/Game/MainBlueprints/Widgets/W_MainMenu.W_MainMenu_C"))
  (`/Game/MainBlueprints/Widgets/W_MainMenu.Launch` _returnvalue_2)
  (`UserWidget.AddToViewport` _returnvalue_2 0))

(event `LevelBegin`
  (bind _returnvalue (`GameplayStatics.GetPlayerController` 0))
  (`WidgetBlueprintLibrary.SetInputMode_GameOnly` _returnvalue)
  (bind _returnvalue_2 (`|CreateWidget` "/Game/MainBlueprints/Widgets/W_MainHUD.W_MainHUD_C" _returnvalue))
  (bind _output_get (set `self.HUD` _returnvalue_2))
  (`UserWidget.AddToViewport` _returnvalue_2 0)
  (`UserWidget.AddToViewport` _output_get 0)
  (bind _asbp_the_gun_panda (cast `/Game/MainBlueprints/Characters/MainCharacter/BP_TheGunPanda` (`GameplayStatics.GetPlayerCharacter` 0)))
  (set `self.PlayerRef` _asbp_the_gun_panda))

(event `InventoryControl`
  (bind _inventoryscreen (`self.InventoryScreen`))
  (if (`self.InventoryOpen`)
    (`/Game/MainBlueprints/Widgets/W_Inventory.UpdateGuns` _inventoryscreen)
    (`Widget.RemoveFromParent` _inventoryscreen)
    (set `self.InventoryOpen` false)
    (`/Game/MainBlueprints/Widgets/W_MainHUD.UpdateGunSet` (`self.HUD`))
    (`WidgetBlueprintLibrary.SetInputMode_GameOnly` (`GameplayStatics.GetPlayerController` 0))
    (else
      (bind _returnvalue (`|CreateWidget` "/Game/MainBlueprints/Widgets/W_Inventory.W_Inventory_C"))
      (`UserWidget.AddToViewport` _returnvalue 0)
      (bind _output_get (set `self.InventoryScreen` _returnvalue))
      (set `self.InventoryOpen` true)
      (`WidgetBlueprintLibrary.SetInputMode_GameAndUIEx` (`GameplayStatics.GetPlayerController` 0) (`|GetArrayItem` (`PanelWidget.GetAllChildren` (`/Game/MainBlueprints/Widgets/W_Inventory.GunInfo` _output_get))) "LockAlways" true true)
      (`Widget.SetKeyboardFocus` _output_get)
      (`Widget.SetKeyboardFocus` (`|GetArrayItem` (`PanelWidget.GetAllChildren` (`/Game/MainBlueprints/Widgets/W_Inventory.GunInfo` _output_get))))))
  (set `PlayerController.bShowMouseCursor` false (`GameplayStatics.GetPlayerController` 0)))

(event `CycleGuns`
  (params (GunToSwitchTo :type Integer))
  (`/Game/MainBlueprints/Widgets/W_MainHUD.SwitchGuns` (`self.HUD`) GunToSwitchTo))

(fn `UserConstructionScript`)