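; Component that makes its owning enemy or interactable a lock-on target and routes incoming hits to it.
; Target and lock events drive the owner's W_LockOn reticule widget, while game mode combat events make non-enemy targets untargetable during combat.
; Damage on enemies is doubled by a status effect (the mark), which it then ends, and is reported as a damage event with debug print.
; Non-enemy owners are treated as interactables and get Shot instead.
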(event `self.ReceiveBeginPlay`
  (`|ExecutionSequence`
    (:`then_0`
      (for _array_element (`Actor.K2_GetComponentsByClass` (`self.GetOwner`) "/Script/UMG.WidgetComponent")
        (bind _asw_lock_on (cast `/Game/MainBlueprints/Widgets/W_LockOn` (`WidgetComponent.GetWidget` _array_element)))
        (set `self.Reticule` _asw_lock_on)))
    (:`then_1`
      (bind _asbp_best_game_mode (cast `/Game/MainBlueprints/BP_BestGameMode` (`GameplayStatics.GetGameMode`)))
      (`|ExecutionSequence`
        (:`then_0`
          (add `/Game/MainBlueprints/BP_BestGameMode.CombatStart` _asbp_best_game_mode (delegate `SwitchOff`)))
        (:`then_1`
          (add `/Game/MainBlueprints/BP_BestGameMode.CombatFinish` _asbp_best_game_mode (delegate `SwitchOn`)))))))

(event `SwitchOff`
  (if (not (`self.Enemy`))
    (set `self.Untargetable` true)))

(event `SwitchOn`
  (set `self.Untargetable` false))

(event `Lock`
  (`/Game/MainBlueprints/Widgets/W_LockOn.Locked` (`self.Reticule`)))

(event `Targeted`
  (`/Game/MainBlueprints/Widgets/W_LockOn.Target` (`self.Reticule`)))

(event `Untargeted`
  (`/Game/MainBlueprints/Widgets/W_LockOn.Untarget` (`self.Reticule`)))

(event `Unlock`
  (`/Game/MainBlueprints/Widgets/W_LockOn.Unlocked` (`self.Reticule`)))

(event `Damage`
  (params (Damage :type "Float (double-precision)") (Stagger :type "Float (double-precision)"))
  (bind _returnvalue (`GameplayStatics.GetPlayerCharacter` 0))
  (if (`self.Enemy`)
    (bind _asenemy_base (cast `/Game/Nick_AI/AI/Enemy_Blueprints/Enemy_base` (`self.GetOwner`)))
    (bind (_value _returnvalue_2) (`BlueprintMapLibrary.Map_Find` (`/Game/Topher/StatusEffectBPCs/BPC_StatusEffectManager.ActiveStatusEffects` (`/Game/Nick_AI/AI/Enemy_Blueprints/Enemy_base.BPC_StatusEffectManager` _asenemy_base)) "NewEnumerator8"))
    (bind _returnvalue_3 (`KismetMathLibrary.SelectFloat` (* 2.0 Damage) Damage _returnvalue_2))
    (`/Game/Nick_AI/AI/Enemy_Blueprints/Enemy_base.Damaged` _asenemy_base _returnvalue_3 Stagger)
    ;[0 0 0] DEBUG
    (`KismetSystemLibrary.PrintString` (`KismetStringLibrary.Concat_StrStr` (`KismetStringLibrary.Conv_DoubleToString` _returnvalue_3) " - " (`KismetStringLibrary.Conv_DoubleToString` Stagger) " - " (`KismetSystemLibrary.GetDisplayName` _asenemy_base)) true true (struct :`G` 0.513873 :`B` 1.0 :`A` 1.0) 5.0)
    (`AISense_Damage.ReportDamageEvent` _asenemy_base _returnvalue _returnvalue_3 (`Actor.K2_GetActorLocation` _returnvalue))
    (if _returnvalue_2
      (`/Game/Topher/StatusEffectBPCs/BPC_StatusEffectParent.EndStatus` _value))
    (else
      (bind _asbp_interactable (cast `/Game/MainBlueprints/Interactables/Interactable/BP_Interactable` (`self.GetOwner`)))
      (`/Game/MainBlueprints/Interactables/Interactable/BP_Interactable.Shot` _asbp_interactable))))