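; BP_FadeableMesh is a static mesh that fades selected material slots out and back in on FadeOut and FadeIn events.
; FadeOut swaps slots listed in FadeableMeshes to a dynamic MI_RadFadeOut instance and drives its FadeAmount by timeline.
; FadeIn reverses a second timeline, then restores the materials cached at BeginPlay.
; Paired DoOnce gates, each reset by the opposite event, block repeated fades in the same direction.
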(event `self.ReceiveBeginPlay`
  (set `self.BaseMaterial` (`MeshComponent.GetMaterials` (`self.StaticMeshComponent`))))

(event `FadeOut`
  (bind _staticmeshcomponent (`self.StaticMeshComponent`))
  (`|ExecutionSequence`
    (:`then_0`
      (`/Engine/EditorBlueprintResources/StandardMacros.DoOnce` false :!label _label
        (:`Completed`
          (bind _returnvalue (`KismetMaterialLibrary.CreateDynamicMaterialInstance` "/Game/MainBlueprints/MaterialStuff/MI_RadFadeOut.MI_RadFadeOut"))
          (bind _output_get (set `self.DynamicMaterial` _returnvalue))
          (for (_ _array_index) (`MeshComponent.GetMaterials` _staticmeshcomponent)
            (if (`KismetArrayLibrary.Array_Contains` (`self.FadeableMeshes`) _array_index)
              (`PrimitiveComponent.SetMaterial` _staticmeshcomponent _array_index _output_get)
              (bind (_direction _newtrack_0) (`Timeline|Timeline` :!via `PlayFromStart`)
                (:`Update`
                  (`MaterialInstanceDynamic.SetScalarParameterValue` _returnvalue "FadeAmount" _newtrack_0))))))))
    (:`then_1`
      (goto _label_2 :!via `Reset`))))

(event `FadeIn`
  (`|ExecutionSequence`
    (:`then_0`
      (`/Engine/EditorBlueprintResources/StandardMacros.DoOnce` false :!label _label_2
        (:`Completed`
          (bind (_direction _newtrack_0) (`Timeline|Timeline_0` :!via `ReverseFromEnd`)
            (:`Update`
              (`MaterialInstanceDynamic.SetScalarParameterValue` (`self.DynamicMaterial`) "FadeAmount" _newtrack_0))
            (:`Finished`
              (for (_array_element _array_index) (`self.BaseMaterial`)
                (`PrimitiveComponent.SetMaterial` (`self.StaticMeshComponent`) _array_index _array_element)))))))
    (:`then_1`
      (goto _label :!via `Reset`))))

(fn `UserConstructionScript`)