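; Drawbridge interactable that drops or swings its bridge when shot, animated by a Timeline.
; On Shot, it calls Unlock on the player's BP_TheGunPanda pawn and destroys its Plank, BPCTarget and LockOn components.
; The Timeline then lerps the bridge's relative roll from its current value toward near zero each update, keeping pitch and yaw.
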(event `self.Shot`
  (bind _bridge (`self.bridge`))
  (bind _relativerotation (`SceneComponent.RelativeRotation` _bridge))
  (bind _asbp_the_gun_panda (cast `/Game/MainBlueprints/Characters/MainCharacter/BP_TheGunPanda` (`GameplayStatics.GetPlayerPawn` 0)))
  (`/Game/MainBlueprints/Characters/MainCharacter/BP_TheGunPanda.Unlock` _asbp_the_gun_panda)
  (`ActorComponent.K2_DestroyComponent` (`self.Plank`))
  (`ActorComponent.K2_DestroyComponent` (`self.BPC_Target`))
  (`ActorComponent.K2_DestroyComponent` (`self.LockOn`))
  (bind (_direction _newtrack_0) (`Timeline|Timeline` :!via `PlayFromStart`)
    (:`Update`
      (`SceneComponent.K2_SetRelativeRotation` _bridge (`KismetMathLibrary.RLerp` _relativerotation (`KismetMathLibrary.MakeRotator` 0.1 (.pitch _relativerotation) (.yaw _relativerotation)) _newtrack_0) false false))))

(fn `UserConstructionScript`
  (`parent.UserConstructionScript`))