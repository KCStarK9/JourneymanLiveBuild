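; BP_Switch is an interactable lever switch that the GunPanda player can toggle or shoot.
; Interacting requires Key01, then flips IsEnabled, snaps the lever's roll and, if a lift is linked, sets its run state and calls the enabled/disabled dispatchers.
; Being shot instead releases the player's lock, removes the targeting components, animates the lever through a timeline and sets SwitchShot, without toggling the lift.
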(event `self.Shot`
  (bind _switch (`self.Switch`))
  (bind _relativerotation (`SceneComponent.RelativeRotation` _switch))
  (bind _asbp_the_gun_panda (cast `/Game/MainBlueprints/Characters/MainCharacter/BP_TheGunPanda` (`GameplayStatics.GetPlayerPawn` 0)))
  (`/Game/MainBlueprints/Characters/MainCharacter/BP_TheGunPanda.Unlock` _asbp_the_gun_panda)
  (`ActorComponent.K2_DestroyComponent` (`self.BPC_Target`))
  (`ActorComponent.K2_DestroyComponent` (`self.LockOn`))
  (bind (_direction _newtrack_0) (`Timeline|Timeline` :!via `PlayFromStart`)
    (:`Update`
      (`SceneComponent.K2_SetRelativeRotation` _switch (`KismetMathLibrary.RLerp` _relativerotation (`KismetMathLibrary.MakeRotator` 25.0 (.pitch _relativerotation) (.yaw _relativerotation)) _newtrack_0) false false)
      (set `self.Switch Shot?` true))))

(fn `SwitchState`
  (bind _switch (`self.Switch`))
  (bind _output_get (set `self.IsEnabled` (not (`self.IsEnabled`))))
  (if _output_get
    (`SceneComponent.K2_SetRelativeRotation` _switch (`KismetMathLibrary.MakeRotator` 20.0) false false)
    (bind _lift_bp (`self.Lift BP`)
      (:`then`
        (`/Game/MainBlueprints/Interactables/Interactable/Children/BP_lift.SetRunState` _lift_bp true)
        (`self.OnEnabled`))
      (:`else`))
    (else
      (`SceneComponent.K2_SetRelativeRotation` _switch (`KismetMathLibrary.MakeRotator` -20.0) false false)
      (bind _lift_bp_2 (`self.Lift BP`)
        (:`then`
          (`/Game/MainBlueprints/Interactables/Interactable/Children/BP_lift.SetRunState` _lift_bp_2 false)
          (`self.OnDisabled`))
        (:`else`)))))

(fn `TryInteract`
  (params (target_character :type "Character Object Reference"))
  (bind _asbp_the_gun_panda (cast `/Game/MainBlueprints/Characters/MainCharacter/BP_TheGunPanda` target_character)
    (:`then`
      (if (`/Game/MainBlueprints/Characters/MainCharacter/BP_TheGunPanda.is_key01_pickup` _asbp_the_gun_panda)
        (`self.SwitchState`)
        (else
          (`KismetSystemLibrary.PrintString` "No key" true true (struct :`R` 1.0 :`G` 0.020908 :`A` 1.0)))))
    (:`CastFailed`
      (`KismetSystemLibrary.PrintString` "Hello"))))

(fn `UserConstructionScript`
  (`parent.UserConstructionScript`))