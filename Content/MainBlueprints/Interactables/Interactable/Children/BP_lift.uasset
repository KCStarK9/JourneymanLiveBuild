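; BP_lift is an interactable lift that moves its static mesh vertically between its base height and TargetLocationZ.
; SetRunState either starts a launch-delay timer or resets the lift and clears both timers.
; Each tick, UpdateLift moves the mesh at constant speed toward the height selected by ShouldDown.
; On reaching TargetLocationZ it starts a fixed close timer, with CloseLift returning it to base.
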(event `CloseLift`
  ;[1 1 1] Close Lift
  (`self.SetRunState` false))

(event `LauncheLift`
  ;[1 1 1] Launche Lift
  (set `self.ShouldDown` true))

(event `self.ReceiveTick`
  (params (DeltaSeconds :type "Float (single-precision)"))
  ;[1 1 1] lift down
  (`self.UpdateLift` DeltaSeconds))

(fn `SetRunState`
  (params (is_down :type Boolean))
  (if is_down
    (if (and (not (`self.ShouldDown`)) (not (`KismetSystemLibrary.K2_IsValidTimerHandle` (`self.LaunchDelayTimer`))))
      (bind _returnvalue (`KismetSystemLibrary.K2_SetTimerDelegate` (`|CreateDelegate` :!event `LauncheLift`) (`self.LaunchDelay`)))
      (set `self.LaunchDelayTimer` _returnvalue))
    (else
      (set `self.ShouldDown` false)
      (`KismetSystemLibrary.K2_ClearAndInvalidateTimerHandle` (`self.LaunchDelayTimer`))
      (`KismetSystemLibrary.K2_ClearAndInvalidateTimerHandle` (`self.CloseLiftDelayTimer`)))))

(fn `UpdateLift`
  (params (DeltaTime :type "Float (double-precision)"))
  (locals (TargetLocZ_Cache :type "Float (double-precision)"))
  (set `local.TargetLocZ_Cache` (`KismetMathLibrary.SelectFloat` (`self.TargetLocationZ`) 0.0 (`self.ShouldDown`)))
  (if (!= (`self.CurLocationZ`) (`local.TargetLocZ_Cache`))
    (bind _output_get (set `self.CurLocationZ` (`KismetMathLibrary.FInterpTo_Constant` (`self.CurLocationZ`) (`local.TargetLocZ_Cache`) DeltaTime 100.0)))
    (`SceneComponent.K2_SetRelativeLocation` (`self.StaticMesh`) (`KismetMathLibrary.MakeVector` 0.0 0.0 _output_get) false false)
    (elif (and (== (`local.TargetLocZ_Cache`) (`self.TargetLocationZ`)) (not (`KismetSystemLibrary.K2_IsValidTimerHandle` (`self.CloseLiftDelayTimer`))))
      (bind _returnvalue (`KismetSystemLibrary.K2_SetTimerDelegate` (`|CreateDelegate` :!event `CloseLift`) 5.0))
      (set `self.CloseLiftDelayTimer` _returnvalue))))

(fn `UserConstructionScript`)