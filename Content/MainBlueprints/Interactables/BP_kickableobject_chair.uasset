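; A kickable chair interactable that guns can push or pull through interface events.
; Push launches the static mesh along the trace direction from start to end, and Pull launches it from its location toward the trace start.
; Both apply a velocity-change impulse, so mass is ignored, scaled by separate push and pull multipliers.
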(event `/Game/Topher/GunInterface.Push`
  (params (TraceStart :type "Vector Structure") (TraceEnd :type "Vector Structure"))
  ;[0 0 0] Interface called by guns to push objects
  (`PrimitiveComponent.AddImpulse` (`self.StaticMesh`) (* (`KismetMathLibrary.GetForwardVector` (`KismetMathLibrary.FindLookAtRotation` TraceStart TraceEnd)) (`self.PushMultplier`)) "None" true))

(event `/Game/Topher/GunInterface.Pull`
  (params (StartTrace :type "Vector Structure"))
  ;[0 0 0] Interface called by guns to pull objects
  (`PrimitiveComponent.AddImpulse` (`self.StaticMesh`) (* (`KismetMathLibrary.GetForwardVector` (`KismetMathLibrary.FindLookAtRotation` (`SceneComponent.K2_GetComponentLocation` (`self.StaticMesh`)) StartTrace)) (`self.PullMultplier`)) "None" true))

(fn `UserConstructionScript`)