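; BP_BestGameMode is a game mode that tracks whether the player is in combat and announces when combat starts and finishes.
; CombatBegin and CombatEnd set the InCombat flag and call the CombatStart and CombatFinish dispatchers.
; Two cross-resetting DoOnce nodes ensure repeated begin or end calls fire only once per transition.
; An unconnected cast to BP_TheGunPanda never runs.
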(event `self.ReceiveBeginPlay`)

(event `CombatBegin`
  (`|ExecutionSequence`
    (:`then_0`
      (`/Engine/EditorBlueprintResources/StandardMacros.DoOnce` false :!label _label
        (:`Completed`
          (set `self.InCombat` true)
          (`self.CombatStart`))))
    (:`then_1`
      (goto _label_2 :!via `Reset`))))

(event `CombatEnd`
  (`|ExecutionSequence`
    (:`then_0`
      (`/Engine/EditorBlueprintResources/StandardMacros.DoOnce` false :!label _label_2
        (:`Completed`
          (set `self.InCombat` false)
          (`self.CombatFinish`))))
    (:`then_1`
      (goto _label :!via `Reset`))))

(fn `UserConstructionScript`)