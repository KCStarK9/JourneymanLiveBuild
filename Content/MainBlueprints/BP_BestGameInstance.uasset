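; BP_BestGameInstance is a Game Instance Blueprint that tracks which of three gun sets the player has equipped.
; The GunSwitch event offsets GunSetActive by the given step, wrapping to the last set below zero and to the first past the end.
; It then assigns the selected set to the EquippedGuns of PlayerRef and prints the active index to screen.
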(event `GunSwitch`
  (params (SwitchInt :type Integer))
  (bind _gunsetactive (`self.GunSetActive`))
  (bind _returnvalue (+ (`self.GunSetActive`) SwitchInt))
  ;[1 1 1] GunSetSwitch
  (if (< _returnvalue 0)
    (set `self.GunSetActive` 2)
    (elif (>= _returnvalue 3)
      (set `self.GunSetActive` 0)
      (else
        (set `self.GunSetActive` _returnvalue))))
  (set `/Game/MainBlueprints/Characters/MainCharacter/BP_TheGunPanda.EquippedGuns` (select `int` _gunsetactive :`0` (`self.GunSet1`) :`1` (`self.GunSet2`) :`2` (`self.GunSet3`)) (`self.PlayerRef`))
  (`KismetSystemLibrary.PrintString` (`KismetStringLibrary.Conv_IntToString` _gunsetactive)))