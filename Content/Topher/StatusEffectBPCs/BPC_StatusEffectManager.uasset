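; Actor component that manages status effects (Freeze, Oil, Slow, Stun, Mark) on its owning Enemy_base.
; BeginPlay builds a duration map from status effect defaults.
; AddStatus resets an active effect's timer or spawns that status's component class on the enemy and tracks it in a map, allowing Freeze and Stun only on staggered enemies.
; ClearStatus removes an effect from that map.
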(event `self.ReceiveBeginPlay`
  (bind (_statuseffectdefaults_freeze _statuseffectdefaults_oil _statuseffectdefaults_slow _statuseffectdefaults_stun _statuseffectdefaults_mark) (break `/Game/Topher/Data/F_StatusEffects` (`self.StatusEffectDefaults`)))
  (set `self.Status Effect Durations` (`|MakeMap` "NewEnumerator5" _statuseffectdefaults_freeze "NewEnumerator6" _statuseffectdefaults_oil "NewEnumerator7" _statuseffectdefaults_slow "NewEnumerator3" _statuseffectdefaults_stun "NewEnumerator8" _statuseffectdefaults_mark :!type "/Game/Topher/Data/E_StatusEffects Enum"))
  (bind _asenemy_base (cast `/Game/Nick_AI/AI/Enemy_Blueprints/Enemy_base` (`self.GetOwner`)))
  (set `self.As Enemy Base` _asenemy_base))

(event `AddStatus`
  (params (Status :type "/Game/Topher/Data/E_StatusEffects Enum" :default "NewEnumerator4") (`IsGunUpgraded?` :type Boolean))
  (bind _status (`self.Status`))
  (bind _as_enemy_base (`self.As Enemy Base`))
  (bind (_value _returnvalue) (`BlueprintMapLibrary.Map_Find` (`self.ActiveStatusEffects`) (`self.Status`)))
  (bind _returnvalue_2 (or (`|EnumEquality` _status "NewEnumerator5") (`|EnumEquality` _status "NewEnumerator3")))
  ;[0 0 0] AddStatus called from BPC_Gun
  (if (`|EnumInequality` Status "NewEnumerator4")
    (set `self.Status` Status)
    (set `self.Is Gun Upgraded?` false)
    ;[0 0 0] Is status effect currently active? If True reset status timer, if False add status.
    (if (or (not _returnvalue_2) (and _returnvalue_2 (`/Game/Nick_AI/AI/Enemy_Blueprints/Enemy_base.Staggered` (`self.As Enemy Base`))))
      (if _returnvalue
        (`/Game/Topher/StatusEffectBPCs/BPC_StatusEffectParent.ResetStatus` _value)
        (else
          (bind _returnvalue_3 (`|AddComponentByClass` _as_enemy_base (`BlueprintMapLibrary.Map_Find` (`self.StatusBPCs`) (`self.Status`)) (`self.Is Gun Upgraded?`) _as_enemy_base (`BlueprintMapLibrary.Map_Find` (`self.Status Effect Durations`) (`self.Status`)) self (`self.Status`)))
          (`BlueprintMapLibrary.Map_Add` (`self.ActiveStatusEffects`) (`self.Status`) _returnvalue_3))))))

(event `ClearStatus`
  (params (StatusToClear :type "/Game/Topher/Data/E_StatusEffects Enum" :default "NewEnumerator4"))
  ;[0 0 0] ClearStatus
  (`BlueprintMapLibrary.Map_Remove` (`self.ActiveStatusEffects`) StatusToClear))