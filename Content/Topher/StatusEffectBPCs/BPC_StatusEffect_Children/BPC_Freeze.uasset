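; BPC_Freeze is a child status effect component that freezes the enemy it is attached to.
; On begin play it sends a stun message to its owner and applies an ice overlay material to the enemy mesh.
; It also looks up one other effect type in the enemy's status effect manager and ends it if active.
; Ending the freeze sends a movement reset message and clears the overlay.
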(event `self.ReceiveBeginPlay`
  (bind (_value _returnvalue) (`BlueprintMapLibrary.Map_Find` (`/Game/Topher/StatusEffectBPCs/BPC_StatusEffectManager.ActiveStatusEffects` (`/Game/Nick_AI/AI/Enemy_Blueprints/Enemy_base.BPC_StatusEffectManager` (`self.As Enemy Base`))) "NewEnumerator0"))
  (`parent.ReceiveBeginPlay`)
  (message `/Game/Topher/GunInterface.Stun` (`self.GetOwner`))
  (`MeshComponent.SetOverlayMaterial` (`Character.Mesh` (`self.As Enemy Base`)) "/Game/Topher/VFX/Overlays/M_OverlayIce.M_OverlayIce")
  (if _returnvalue
    (`self.EndStatus` _value)))

(event `self.EndStatus`
  (`parent.EndStatus`)
  (message `/Game/Topher/GunInterface.ResetMovement` (`self.GetOwner`))
  (`MeshComponent.SetOverlayMaterial` (`Character.Mesh` (`self.As Enemy Base`)) null))