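; BPC_Oil is a child status effect component that oils its owner, slowing it while the effect lasts.
; On BeginPlay it sends SlowMessage to the owner and applies the oil overlay material to the enemy mesh before calling the parent logic.
; EndStatus sends ResetMovementMessage and clears the overlay, then defers to the parent.
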(event `self.ReceiveBeginPlay`
  (message `/Game/Topher/GunInterface.Slow` (`self.GetOwner`))
  (`MeshComponent.SetOverlayMaterial` (`Character.Mesh` (`self.As Enemy Base`)) "/Game/Topher/VFX/Overlays/M_OverlayOil.M_OverlayOil")
  (`parent.ReceiveBeginPlay`))

(event `self.EndStatus`
  (message `/Game/Topher/GunInterface.ResetMovement` (`self.GetOwner`))
  (`MeshComponent.SetOverlayMaterial` (`Character.Mesh` (`self.As Enemy Base`)) null)
  (`parent.EndStatus`))