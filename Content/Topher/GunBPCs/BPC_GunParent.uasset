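; BPC_GunParent is the parent gun component, handling firing, effects and damage for its owner, cast as the Gun Panda or an enemy.
; ShootGun blocks refiring until RollReload, plays sound and spawns a Niagara trail from alternating muzzles to the target or straight ahead.
; With a target, it combines child-set, base, bonus and GunManager upgrade-dependent values into damage and stagger, applied through the Gun Panda reference.
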(event `self.ReceiveBeginPlay`
  (bind _returnvalue (`self.GetOwner`))
  (add `/Game/Topher/GunBPCs/BPC_GunManager.ReloadAllGuns` (`self.GunManager`) (`|CreateDelegate` :!event `RollReload`))
  (bind _asbp_the_gun_panda (cast `/Game/MainBlueprints/Characters/MainCharacter/BP_TheGunPanda` _returnvalue)
    (:`then`
      (set `self.As BP The Gun Panda` _asbp_the_gun_panda))
    (:`CastFailed`
      (bind _asenemy_base (cast `/Game/Nick_AI/AI/Enemy_Blueprints/Enemy_base` _returnvalue))
      (set `self.As Enemy Base` _asenemy_base))))

(event `RollReload`
  ;[0 0 0] Roll Reload
  (set `self.CanBeFired` true))

(event `ShootGun`
  (params (TargetEnemy :type "Actor Object Reference") (MuzzleOneTransform :type "Transform Structure") (MuzzleTwoTransform :type "Transform Structure") (ActiveGun :type Integer) (HasTarget :type Boolean))
  (bind ((`BuilletTrail_8_3C047621499F891563A5A48707720D77` _buillettrail) (`BulletImpact_11_1A71D4C245C19820810C258599857B10` _bulletimpact)) (break `/Game/Topher/Data/F_GunFX` (`self.GunFX`)))
  (bind (_returnvalue_location _returnvalue_rotation) (`KismetMathLibrary.BreakTransform` (`KismetMathLibrary.SelectTransform` MuzzleOneTransform MuzzleTwoTransform (== (mod ActiveGun 2) 1))))
  ;[0 0 0] Shoot Gun
  (if HasTarget
    (set `self.Target Enemy` TargetEnemy))
  (set `self.CanBeFired` false)
  (`|ExecutionSequence`
    (:`then_0`
      ;[1 1 1] Bang
      (`GameplayStatics.PlaySoundAtLocation` "/Game/MainBlueprints/SoundAssets/Shot_3.Shot_3" (`Actor.K2_GetActorLocation` (`self.As BP The Gun Panda`)) (struct) 1.0 1.0 0.0 null null null null))
    (:`then_1`
      (`self.SpawnVFX` _returnvalue_location _returnvalue_rotation _buillettrail _bulletimpact)
      (if HasTarget
        (`self.CalculateDamage`)))))

(event `CalculateDamage`
  ;[0 0 0] Caluculate and apply damage
  (`self.DamageAndStaggerCalculation`)
  (`/Game/MainBlueprints/Characters/MainCharacter/BP_TheGunPanda.Apply Damage` (`self.As BP The Gun Panda`) (`self.Damage`) (`self.Stagger`) (`.statusEffect_5_9A357DB14C38F9C04E5933A01F14787C` (break `/Game/Topher/Data/F_Gun` (`self.GunInfo`))) (`self.IsUpgraded?`))
  (set `self.Damage` 0.0)
  (set `self.Stagger` 0.0)
  (set `self.Target Enemy` null))

(fn `DamageAndStaggerCalculation`
  (bind ((`gunName_13_7C4A01CA453754A66F4EFE85F4179906` _gunname) (`BasicDamage_37_C39876C24C3474862D83E7B52410AD6C` _basicdamage) (`UpgradeDamage_61_069B49C14D46E62606150DB4D55686F4` _upgradedamage)) (break `/Game/Topher/Data/F_Gun` (`self.GunInfo`)))
  (bind ((`StaggerDamage_39_E32A9290467E1174E0231C8FCB0181A0` _staggerdamage) (`UpgradeStagger_66_26B906494557CC9DBF7244BA069AF0FA` _upgradestagger)) (break `/Game/Topher/Data/F_Gun` (`self.GunInfo`)))
  (bind _returnvalue (not (`BlueprintMapLibrary.Map_Find` (`/Game/Topher/GunBPCs/BPC_GunManager.GunUpgradeStatus` (`self.GunManager`)) _gunname)))
  (set `self.Damage` (+ (`self.Damage`) (`.BasicDamage_37_C39876C24C3474862D83E7B52410AD6C` (break `/Game/Topher/Data/F_Gun` (`self.GunInfo`))) (`KismetMathLibrary.SelectFloat` (`.BonusDamage_48_92EA5EFD405F8FB5E62DFE8FC7524950` (break `/Game/Topher/Data/F_Gun` (`self.GunInfo`))) 0.0 (`self.DealBonusDamage?`)) (`KismetMathLibrary.SelectFloat` 0.0 _upgradedamage _returnvalue)))
  (set `self.Stagger` (+ (`self.Stagger`) (`KismetMathLibrary.SelectFloat` _staggerdamage _upgradestagger _returnvalue)))
  (return))

(fn `SetBeamEnd`
  (params (NiagaraSystem :type "FXSystemComponent Object Reference") (MuzzleLocation :type "Vector Structure") (MuzzleRotation :type "Rotator Structure"))
  (`self.Target Enemy`
    (:`then`
      (`FXSystemComponent.SetVectorParameter` NiagaraSystem "BeamEnd" (`Actor.K2_GetActorLocation` (`self.Target Enemy`))))
    (:`else`
      (`FXSystemComponent.SetVectorParameter` NiagaraSystem "BeamEnd" (+ MuzzleLocation (* (`KismetMathLibrary.GetForwardVector` MuzzleRotation) 5000.0))))))

(fn `SpawnVFX`
  (params (MuzzleLocation :type "Vector Structure") (MuzzleRotation :type "Rotator Structure") (BulletTrail :type "NiagaraSystem Object Reference") (BulletImpact :type "NiagaraSystem Object Reference"))
  (bind _returnvalue (`NiagaraFunctionLibrary.SpawnSystemAtLocation` BulletTrail MuzzleLocation MuzzleRotation (1.0 1.0 1.0) false))
  (`self.SetBeamEnd` _returnvalue MuzzleLocation MuzzleRotation)
  (bind _target_enemy (`self.Target Enemy`)
    (:`then`
      (`NiagaraFunctionLibrary.SpawnSystemAtLocation` BulletImpact (`Actor.K2_GetActorLocation` _target_enemy) (struct) (1.0 1.0 1.0) false))
    (:`else`)))