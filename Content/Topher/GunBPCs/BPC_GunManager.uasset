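; Player component that manages an ordered set of guns, equipping a default four on BeginPlay and handling set swaps, firing and roll reload.
; AddGun builds each gun component from info and FX data tables.
; Each successful shot advances the active gun and HUD until the last wraps to first, while the alternating right/left hand mesh and Niagara effect preview the gun two slots ahead.
; RollReload reloads all guns and resets the cycle.
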(event `self.ReceiveBeginPlay`
  ;[0 0 0] Adds guns to player on spawn
  (`self.SwitchGunSet` (`|MakeArray` "NewEnumerator0" "NewEnumerator9" "NewEnumerator10" "NewEnumerator5" :!type "/Game/Topher/Data/E_GunNames Enum")))

(event `SwitchGunSet`
  (params (`Gun Set` :type "Array of /Game/Topher/Data/E_GunNames Enum"))
  ;[0 0 0] Gun set switching
  (bind _output_get (set `self.NewGunSet` `Gun Set`))
  (for _array_element (`self.CurrentGunSet`)
    (`self.RemoveGun` _array_element))
  (bind _output_get_2 (set `self.CurrentGunSet` _output_get))
  (for _array_element_2 _output_get_2
    (`self.Add Gun` _array_element_2)))

(event `Add Gun`
  (params (Gun :type "/Game/Topher/Data/E_GunNames Enum" :default "NewEnumerator4"))
  (bind _value (`BlueprintMapLibrary.Map_Find` (`self.DataTableRows`) Gun))
  ;[0 0 0] Add gun to Guns Map and Gun Order Array
  (bind _returnvalue (`|GetDataTableRow` "/Game/Topher/Data/DT_GunInfo.DT_GunInfo" (`.RowName` (break `DataTableRowHandle` _value)))
    (:`then`
      (bind _returnvalue_2 (`|GetDataTableRow` "/Game/Topher/Data/DT_GunFX.DT_GunFX" (`.RowName` (break `DataTableRowHandle` _value)))
        (:`then`
          (bind (_gunname _gunclass) (break `/Game/Topher/Data/F_Gun` _returnvalue))
          (bind _returnvalue_3 (`|AddComponentByClass` :`self` (`self.GetOwner`) :`Class` _gunclass :`GunFX` _returnvalue_2 :`GunManager` self))
          (`BlueprintMapLibrary.Map_Add` (`self.AquiredGuns`) _gunname _returnvalue_3)
          (`KismetArrayLibrary.Array_AddUnique` (`self.CurrentGunSet`) _gunname)
          (`BlueprintMapLibrary.Map_Add` (`self.GunVFX`) _gunname (`.GunPassive_17_68D2715D41DE7D03B83D98B1DA185246` (break `/Game/Topher/Data/F_GunFX` _returnvalue_2)))
          (bind _returnvalue_4 (`KismetArrayLibrary.Array_Find` (`self.CurrentGunSet`) _gunname))
          (if (or (== _returnvalue_4 0) (== _returnvalue_4 1))
            (`self.SetPassiveVFX` _returnvalue_4)
            (`self.SetGunMesh` _returnvalue_4)))))))

(event `ShootGun`
  (params (MuzzleOneTransform :type "Transform Structure") (MuzzleTwoTransform :type "Transform Structure") (TargetEnemy :type "Actor Object Reference") (HasTarget :type Boolean))
  (bind _value (`BlueprintMapLibrary.Map_Find` (`self.AquiredGuns`) (`|GetArrayItem` (`self.CurrentGunSet`) (`self.ActiveGun`))))
  ;[0 0 0] Shoot Gun
  (set `self.Muzzle One Transform` MuzzleOneTransform)
  (set `self.Muzzle Two Transform` MuzzleTwoTransform)
  (if HasTarget
    (set `self.TargetEnemy` TargetEnemy))
  ;;[0 0 0] If player has guns
  (if (> (`KismetArrayLibrary.Array_Length` (`self.CurrentGunSet`)) 0)
    ;;[0 0 0] If current gun can be fired, shoot gun
    (if (and (`KismetSystemLibrary.IsValid` _value) (`/Game/Topher/GunBPCs/BPC_GunParent.CanBeFired` _value))
      (`/Game/Topher/GunBPCs/BPC_GunParent.ShootGun` _value (`self.TargetEnemy`) (`self.Muzzle One Transform`) (`self.Muzzle Two Transform`) (`self.ActiveGun`) HasTarget)
      ;;[0 0 0] Update Gun VFX
      (`self.SetPassiveVFX` (+ (`self.ActiveGun`) 2))
      ;;[0 0 0] Update Gun Mesh
      (`self.SetGunMesh` (+ (`self.ActiveGun`) 2))
      ;;[0 0 0] If all guns have been fired, start reload
      (if (< (`self.ActiveGun`) (- (`KismetArrayLibrary.Array_Length` (`self.CurrentGunSet`)) 1))
        (bind _result (`/Engine/EditorBlueprintResources/StandardMacros.IncrementInt` (`self.ActiveGun`))
          (:`  `
            (bind _asbp_best_hud (cast `/Game/MainBlueprints/BP_BestHUD` (`PlayerController.GetHUD` (`GameplayStatics.GetPlayerController` 0))))
            (`/Game/MainBlueprints/BP_BestHUD.CycleGuns` _asbp_best_hud _result)
            (`KismetSystemLibrary.Delay` 0.2)
            (`GameplayStatics.PlaySound2D` "/Game/MainBlueprints/SoundAssets/Draw.Draw" 1.0 1.0 0.0 null null)))
        (else
          (set `self.ActiveGun` 0)))
      (else
        (`GameplayStatics.PlaySound2D` "/Game/MainBlueprints/SoundAssets/Click.Click" 1.0 1.0 0.0 null null)))))

(event `RollReload`
  ;[0 0 0] Roll Reload
  ;;[0 0 0] Calls RollReload in all guns
  (`self.ReloadAllGuns`)
  (set `self.ActiveGun` 0)
  (bind _asbp_best_hud (cast `/Game/MainBlueprints/BP_BestHUD` (`PlayerController.GetHUD` (`GameplayStatics.GetPlayerController` 0))))
  (`/Game/MainBlueprints/BP_BestHUD.CycleGuns` _asbp_best_hud 0)
  (for _index (range 2)
    ;;[0 0 0] Update Gun VFX
    (`self.SetPassiveVFX` _index)
    ;;[0 0 0] Update Gun Mesh
    (`self.SetGunMesh` _index)))

(fn `GetGunMeshComponent`
  (params (Tag :type Name))
  (returns (Output :type "StaticMeshComponent Object Reference"))
  (return (`|GetArrayItem` (`Actor.GetComponentsByTag` (`self.GetOwner`) "/Script/Engine.StaticMeshComponent" Tag))))

(fn `GetPassiveEffectComponent`
  (params (Tag :type Name))
  (returns (Output :type "NiagaraComponent Object Reference"))
  (return (`|GetArrayItem` (`Actor.GetComponentsByTag` (`self.GetOwner`) "/Script/Niagara.NiagaraComponent" Tag))))

(fn `RemoveGun`
  (params (GunToRemove :type "/Game/Topher/Data/E_GunNames Enum (by ref)"))
  (`self.K2_DestroyComponent` (`BlueprintMapLibrary.Map_Find` (`self.AquiredGuns`) (`local.GunToRemove`)))
  (`BlueprintMapLibrary.Map_Remove` (`self.AquiredGuns`) (`local.GunToRemove`))
  (`KismetArrayLibrary.Array_RemoveItem` (`self.CurrentGunSet`) (`local.GunToRemove`))
  (return))

(fn `SetGunMesh`
  (params (GunIndex :type Integer))
  (bind _output (`self.GetGunMeshComponent` "GunLeft"))
  (bind _output_2 (`self.GetGunMeshComponent` "GunRight"))
  (bind _returnvalue (`|GetDataTableRow` "/Game/Topher/Data/DT_GunInfo.DT_GunInfo" (`.RowName` (break `DataTableRowHandle` (`BlueprintMapLibrary.Map_Find` (`self.DataTableRows`) (`|GetArrayItem` (`self.CurrentGunSet`) GunIndex)))))
    (:`then`
      (if (!= (mod GunIndex 2) 1)
        (bind ((`Mesh_56_5C57CAB84869F51E0BAD8EA256B04886` _mesh) (`Material_72_4FFFEF304C1D4C79ECC58086812E0FE7` _material)) (break `/Game/Topher/Data/F_Gun` _returnvalue))
        (`StaticMeshComponent.SetStaticMesh` _output_2 _mesh)
        (`PrimitiveComponent.SetMaterial` _output_2 0 _material)
        (else
          (`StaticMeshComponent.SetStaticMesh` _output _mesh)
          (`PrimitiveComponent.SetMaterial` _output 0 _material))))))

(fn `SetPassiveVFX`
  (params (GunIndex :type Integer))
  (bind _returnvalue (select `bool` (> (`local.GunIndex`) 3) :`false` (`BlueprintMapLibrary.Map_Find` (`self.GunVFX`) (`|GetArrayItem` (`self.CurrentGunSet`) GunIndex))))
  (if (!= (mod GunIndex 2) 1)
    (`NiagaraComponent.SetAsset` (`self.GetPassiveEffectComponent` "PassiveRight") _returnvalue true)
    (else
      (`NiagaraComponent.SetAsset` (`self.GetPassiveEffectComponent` "PassiveLeft") _returnvalue true))))