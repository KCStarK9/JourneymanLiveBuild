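; Swap-lock gun component, a child gun Blueprint that swaps the player panda's position with the targeted enemy's.
; It overrides CalculateDamage, acting only when the target is valid and has a status effect manager.
; It adds a non-upgraded status, teleports the player to the enemy's location and rotation and the enemy to the player's old location, then runs the parent damage calculation.
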(event `self.CalculateDamage`
  (bind _target_enemy (`self.Target Enemy`))
  (bind _target_enemy_2 (`self.Target Enemy`)
    (:`then`
      (bind _returnvalue (`Actor.GetComponentByClass` _target_enemy_2 "/Game/Topher/StatusEffectBPCs/BPC_StatusEffectManager.BPC_StatusEffectManager_C"))
      (if (`KismetSystemLibrary.IsValid` _returnvalue)
        (`/Game/Topher/StatusEffectBPCs/BPC_StatusEffectManager.AddStatus` _returnvalue "NewEnumerator3" false)
        (set `self.PlayerLocation` (`Actor.K2_GetActorLocation` (`self.As BP The Gun Panda`)))
        (`Actor.K2_SetActorLocationAndRotation` (`self.As BP The Gun Panda`) (`Actor.K2_GetActorLocation` _target_enemy) (`Actor.K2_GetActorRotation` _target_enemy) false true)
        (`Actor.K2_SetActorLocation` (`self.Target Enemy`) (`self.PlayerLocation`) false true)
        (`parent.CalculateDamage`)))
    (:`else`)))