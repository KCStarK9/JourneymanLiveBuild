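; Scope-lock gun component, a child gun Blueprint whose shot damage scales with how long it is charged.
; UpdateCharge stores charge time as a ratio capped at one while its gun type is active and charging, and debug-prints it.
; ShootGun calls the parent, then applies basic plus charge-scaled bonus damage and stagger through the target's BPC_Target component.
; CalculateDamage is overridden but empty.
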(event `UpdateCharge`
  (params (IsCharging :type Boolean) (CurrentCharge :type "Float (double-precision)"))
  (bind _gunmanager (`self.GunManager`))
  (if (and (`|EnumEquality` (`|GetArrayItem` (`/Game/Topher/GunBPCs/BPC_GunManager.CurrentGunSet` _gunmanager) (`/Game/Topher/GunBPCs/BPC_GunManager.ActiveGun` _gunmanager)) "NewEnumerator11") IsCharging)
    (bind _output_get (set `self.Charge amount` (`KismetMathLibrary.FMin` (/ CurrentCharge (`self.MaxChargeTime`)) 1.0)))
    (`KismetSystemLibrary.PrintString` (`KismetStringLibrary.Conv_DoubleToString` _output_get) true true (struct :`G` 0.66 :`B` 1.0 :`A` 1.0) 0.0)))

(event `self.ShootGun`
  (params (TargetEnemy :type "Actor Object Reference") (MuzzleOneTransform :type "Transform Structure") (MuzzleTwoTransform :type "Transform Structure") (ActiveGun :type Integer) (HasTarget :type Boolean))
  (bind ((`BasicDamage_37_C39876C24C3474862D83E7B52410AD6C` _basicdamage) (`BonusDamage_48_92EA5EFD405F8FB5E62DFE8FC7524950` _bonusdamage) (`StaggerDamage_39_E32A9290467E1174E0231C8FCB0181A0` _staggerdamage)) (break `/Game/Topher/Data/F_Gun` (`self.GunInfo`)))
  (bind _returnvalue (`Actor.GetComponentByClass` (`self.Target Enemy`) "/Game/MainBlueprints/BPComponents/BPC_Target.BPC_Target_C"))
  (`parent.ShootGun` TargetEnemy MuzzleOneTransform MuzzleTwoTransform ActiveGun HasTarget)
  (if (`KismetSystemLibrary.IsValid` _returnvalue)
    (`/Game/MainBlueprints/BPComponents/BPC_Target.Damage` _returnvalue (+ _basicdamage (* _bonusdamage (`self.Charge amount`))) _staggerdamage)
    (set `self.Target Enemy` null)
    (set `self.Damage` 0.0)
    (set `self.Stagger` 0.0)))

(event `self.CalculateDamage`)