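; Shatter-lock gun component that deals basic damage to its target and triggers an area burst when that target carries a specific status effect.
; On damage calculation, it checks the target's BPC_StatusEffectManager and, if the status is active, ends it and flags bonus damage.
; A debug-drawn sphere trace at the target then gathers unique pawns, applying bonus and stagger damage through their BPC_Target components.
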(event `self.CalculateDamage`
  (bind ((`BonusDamage_48_92EA5EFD405F8FB5E62DFE8FC7524950` _bonusdamage) (`StaggerDamage_39_E32A9290467E1174E0231C8FCB0181A0` _staggerdamage)) (break `/Game/Topher/Data/F_Gun` (`self.GunInfo`)))
  (bind _returnvalue (`Actor.K2_GetActorLocation` (`self.Target Enemy`)))
  (bind (_value _returnvalue_2) (`BlueprintMapLibrary.Map_Find` (`/Game/Topher/StatusEffectBPCs/BPC_StatusEffectManager.ActiveStatusEffects` (`Actor.GetComponentByClass` (`self.Target Enemy`) "/Game/Topher/StatusEffectBPCs/BPC_StatusEffectManager.BPC_StatusEffectManager_C")) "NewEnumerator5"))
  (if _returnvalue_2
    (set `self.DealBonusDamage?` true)
    (`/Game/Topher/StatusEffectBPCs/BPC_StatusEffectParent.EndStatus` _value)
    (`self.DealBasicDamage`)
    (bind _outhits (`KismetSystemLibrary.SphereTraceMultiForObjects` :`Start` _returnvalue :`End` _returnvalue :`Radius` (`self.AOERadius`) :`ObjectTypes` (`|MakeArray` "ObjectTypeQuery3" :!type "EObjectTypeQuery Enum") :`DrawDebugType` "ForDuration" :`TraceColor` (struct :`G` 0.183846 :`B` 1.0 :`A` 1.0) :`TraceHitColor` (struct :`R` 1.0 :`G` 0.869988 :`A` 1.0) :`DrawTime` 0.5))
    (for _array_element _outhits
      (`KismetArrayLibrary.Array_AddUnique` (`self.Hit Actor`) (`.HitActor` (`GameplayStatics.BreakHitResult` _array_element))))
    (set `self.Target Enemy` null)
    (set `self.Damage` 0.0)
    (set `self.Stagger` 0.0)
    (for _array_element_2 (`self.Hit Actor`)
      (bind _returnvalue_3 (`Actor.GetComponentByClass` _array_element_2 "/Game/MainBlueprints/BPComponents/BPC_Target.BPC_Target_C"))
      (if (`KismetSystemLibrary.IsValid` _returnvalue_3)
        (`/Game/MainBlueprints/BPComponents/BPC_Target.Damage` _returnvalue_3 _bonusdamage _staggerdamage)))
    (`KismetArrayLibrary.Array_Clear` (`self.Hit Actor`))
    (else
      (set `self.DealBonusDamage?` false)
      (`self.DealBasicDamage`))))

(fn `DealBasicDamage`
  (`/Game/MainBlueprints/BPComponents/BPC_Target.Damage` (`Actor.GetComponentByClass` (`self.Target Enemy`) "/Game/MainBlueprints/BPComponents/BPC_Target.BPC_Target_C") (`.BasicDamage_37_C39876C24C3474862D83E7B52410AD6C` (break `/Game/Topher/Data/F_Gun` (`self.GunInfo`))) 0.0))