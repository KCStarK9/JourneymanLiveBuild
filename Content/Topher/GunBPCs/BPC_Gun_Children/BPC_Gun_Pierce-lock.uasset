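; Pierce-lock gun component that overrides damage calculation so a shot hits every target along a line.
; A multi sphere trace runs forward from the Gun Panda actor over the gun's range, with debug drawing on, collecting unique BPC_Target components from pawns.
; Each target takes stagger and basic damage, plus bonus damage scaled by its index in the hit list.
; The target list and locked enemy are then cleared.
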(event `self.CalculateDamage`
  (bind _as_bp_the_gun_panda (`self.As BP The Gun Panda`))
  (bind ((`BasicDamage_37_C39876C24C3474862D83E7B52410AD6C` _basicdamage) (`BonusDamage_48_92EA5EFD405F8FB5E62DFE8FC7524950` _bonusdamage) (`StaggerDamage_39_E32A9290467E1174E0231C8FCB0181A0` _staggerdamage)) (break `/Game/Topher/Data/F_Gun` (`self.GunInfo`)))
  (bind _returnvalue (`Actor.K2_GetActorLocation` _as_bp_the_gun_panda))
  (bind _outhits (`KismetSystemLibrary.SphereTraceMultiForObjects` :`Start` _returnvalue :`End` (+ _returnvalue (* (`Actor.GetActorForwardVector` _as_bp_the_gun_panda) (`.gunRange_10_99A68C41477E98F5322A408389DC9AE8` (break `/Game/Topher/Data/F_Gun` (`self.GunInfo`))))) :`Radius` 10.0 :`ObjectTypes` (`|MakeArray` "ObjectTypeQuery3" :!type "EObjectTypeQuery Enum") :`DrawDebugType` "ForDuration"))
  (for _array_element _outhits
    (bind _returnvalue_2 (`Actor.GetComponentByClass` (`.HitActor` (`GameplayStatics.BreakHitResult` _array_element)) "/Game/MainBlueprints/BPComponents/BPC_Target.BPC_Target_C"))
    (if (`KismetSystemLibrary.IsValid` _returnvalue_2)
      (`KismetArrayLibrary.Array_AddUnique` (`self.Targets`) _returnvalue_2)))
  (for (_array_element_2 _array_index) (`self.Targets`)
    (`/Game/MainBlueprints/BPComponents/BPC_Target.Damage` _array_element_2 (+ _basicdamage (* _bonusdamage _array_index)) _staggerdamage))
  (set `self.Target Enemy` null)
  (`KismetArrayLibrary.Array_Clear` (`self.Targets`)))