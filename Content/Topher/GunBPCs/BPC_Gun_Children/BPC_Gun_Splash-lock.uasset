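; BPC_Gun_Splash-lock is a child gun component that fires a cone-shaped splash attack, damaging every target in front of the gun's owning panda.
; After the parent shot, it sweeps capsule traces across the cone in five-degree yaw steps, collecting unique BPC_Target components and ignoring actors already hit.
; Each target takes the gun's basic and stagger damage once, with an empty CalculateDamage override suppressing the parent's damage calculation.
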(event `self.ShootGun`
  (params (TargetEnemy :type "Actor Object Reference") (MuzzleOneTransform :type "Transform Structure") (MuzzleTwoTransform :type "Transform Structure") (ActiveGun :type Integer) (HasTarget :type Boolean))
  (bind _conedegrees (`self.ConeDegrees`))
  (bind _as_bp_the_gun_panda (`self.As BP The Gun Panda`))
  (bind ((`BasicDamage_37_C39876C24C3474862D83E7B52410AD6C` _basicdamage) (`StaggerDamage_39_E32A9290467E1174E0231C8FCB0181A0` _staggerdamage)) (break `/Game/Topher/Data/F_Gun` (`self.GunInfo`)))
  (bind _returnvalue (`Actor.K2_GetActorLocation` _as_bp_the_gun_panda))
  (`parent.ShootGun` TargetEnemy MuzzleOneTransform MuzzleTwoTransform ActiveGun HasTarget)
  (set `self.VectorRotationAmount` (* _conedegrees -0.5))
  (for _ (range 1 (+ (/ _conedegrees 5.0) 1))
    (bind _outhits (`KismetSystemLibrary.CapsuleTraceMultiForObjects` _returnvalue (+ _returnvalue (* (`KismetMathLibrary.GreaterGreater_VectorRotator` (`Actor.GetActorForwardVector` _as_bp_the_gun_panda) (`KismetMathLibrary.MakeRotator` 0.0 0.0 (`self.VectorRotationAmount`))) (`.gunRange_10_99A68C41477E98F5322A408389DC9AE8` (break `/Game/Topher/Data/F_Gun` (`self.GunInfo`))))) 35.0 90.0 (`|MakeArray` "ObjectTypeQuery3" "ObjectTypeQuery2" :!type "EObjectTypeQuery Enum") false (`self.Actors to Ignore`) "ForDuration" true (struct :`R` 1.0 :`A` 1.0) (struct :`G` 1.0 :`A` 1.0) 0.5))
    (for _array_element _outhits
      (bind (_bblockinghit _binitialoverlap _time _distance _location _impactpoint _normal _impactnormal _physmat _hitactor) (`GameplayStatics.BreakHitResult` _array_element))
      (`KismetArrayLibrary.Array_AddUnique` (`self.Actors to Ignore`) _hitactor)
      (bind _returnvalue_2 (`Actor.GetComponentByClass` _hitactor "/Game/MainBlueprints/BPComponents/BPC_Target.BPC_Target_C"))
      (if (`KismetSystemLibrary.IsValid` _returnvalue_2)
        (`KismetArrayLibrary.Array_AddUnique` (`self.Targets`) _returnvalue_2)))
    (set `self.VectorRotationAmount` (+ (`self.VectorRotationAmount`) 5.0)))
  (for _array_element_2 (`self.Targets`)
    (`/Game/MainBlueprints/BPComponents/BPC_Target.Damage` _array_element_2 _basicdamage _staggerdamage))
  (`KismetArrayLibrary.Array_Clear` (`self.Targets`))
  (`KismetArrayLibrary.Array_Clear` (`self.Actors to Ignore`))
  (set `self.Damage` 0.0)
  (set `self.Stagger` 0.0)
  (set `self.Target Enemy` null))

(event `self.CalculateDamage`
  ;[0 0 0] Stop parent calculate damage
)