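; Skill-lock gun component whose shot damages the target enemy, then ricochets between nearby targets up to a maximum bounce count.
; Each bounce recursively sphere-traces around the current target, ignoring previous victims, and applies gun damage and stagger through the hit actor's BPC_Target.
; The trace searches Pawns first, switching to WorldDynamic objects when none are found, and draws debug spheres.
; A hit lacking BPC_Target ends the chain.
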(event `Ricochet`
  (bind ((`BasicDamage_37_C39876C24C3474862D83E7B52410AD6C` _basicdamage) (`StaggerDamage_39_E32A9290467E1174E0231C8FCB0181A0` _staggerdamage)) (break `/Game/Topher/Data/F_Gun` (`self.GunInfo`)))
  (bind _returnvalue (`Actor.K2_GetActorLocation` (`self.CurrentTarget`)))
  (if (<= (`self.RicochetCount`) (`self.MaxRicochets`)) :!label _label
    (`KismetArrayLibrary.Array_AddUnique` (`self.ActorsToIgnore`) (`self.CurrentTarget`))
    (bind (_outhit _returnvalue_2) (`KismetSystemLibrary.SphereTraceSingleForObjects` _returnvalue _returnvalue (`self.AOERadius`) (`|MakeArray` (`self.Object Type`)) false (`self.ActorsToIgnore`) "ForDuration" true (struct :`G` 0.233537 :`B` 1.0 :`A` 1.0) (struct :`R` 1.0 :`G` 0.910243 :`A` 1.0) 2.0))
    (if _returnvalue_2
      (bind (_bblockinghit _binitialoverlap _time _distance _location _impactpoint _normal _impactnormal _physmat _hitactor) (`GameplayStatics.BreakHitResult` _outhit))
      (if (`KismetSystemLibrary.IsValid` (`Actor.GetComponentByClass` _hitactor "/Game/MainBlueprints/BPComponents/BPC_Target.BPC_Target_C"))
        (set `self.CurrentTarget` _hitactor)
        (`/Engine/EditorBlueprintResources/StandardMacros.IncrementInt` (`self.RicochetCount`)
          (:`  `
            (`/Game/MainBlueprints/BPComponents/BPC_Target.Damage` (`Actor.GetComponentByClass` (`self.CurrentTarget`) "/Game/MainBlueprints/BPComponents/BPC_Target.BPC_Target_C") _basicdamage _staggerdamage)
            (`self.Ricochet`))))
      (elif (`|EnumEquality` (`self.Object Type`) "ObjectTypeQuery2")
        (`self.ResetVariables`)
        (else
          (set `self.Object Type` "ObjectTypeQuery2")
          (`self.Ricochet`))))
    (else
      (`self.ResetVariables`))))

(event `self.CalculateDamage`
  (bind ((`BasicDamage_37_C39876C24C3474862D83E7B52410AD6C` _basicdamage) (`StaggerDamage_39_E32A9290467E1174E0231C8FCB0181A0` _staggerdamage)) (break `/Game/Topher/Data/F_Gun` (`self.GunInfo`)))
  (`self.ResetVariables`)
  (set `self.CurrentTarget` (`self.Target Enemy`))
  (set `self.Target Enemy` null)
  (`/Game/MainBlueprints/BPComponents/BPC_Target.Damage` (`Actor.GetComponentByClass` (`self.CurrentTarget`) "/Game/MainBlueprints/BPComponents/BPC_Target.BPC_Target_C") _basicdamage _staggerdamage)
  (goto _label))

(event `ResetVariables`
  (set `self.CurrentTarget` null)
  (set `self.RicochetCount` 0)
  (`KismetArrayLibrary.Array_Clear` (`self.ActorsToIgnore`))
  (set `self.Object Type` "ObjectTypeQuery3"))