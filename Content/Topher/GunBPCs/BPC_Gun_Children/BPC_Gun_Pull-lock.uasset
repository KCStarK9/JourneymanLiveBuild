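; Gun component for the Pull-lock weapon, which adds an area pull and a status effect to each shot.
; After the parent shot logic, it centers a multi-sphere trace on the target, or on a forward sphere trace's hit point when untargeted.
; Each unique actor hit receives a status through its status effect manager and a GunInterface pull message carrying the area's center.
; The area trace draws a brief debug sphere.
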(event `self.ShootGun`
  (params (TargetEnemy :type "Actor Object Reference") (MuzzleOneTransform :type "Transform Structure") (MuzzleTwoTransform :type "Transform Structure") (ActiveGun :type Integer) (HasTarget :type Boolean))
  (bind _hit_actor (`self.Hit Actor`))
  (bind _as_bp_the_gun_panda (`self.As BP The Gun Panda`))
  (bind _returnvalue (`Actor.K2_GetActorLocation` _as_bp_the_gun_panda))
  (`parent.ShootGun` TargetEnemy MuzzleOneTransform MuzzleTwoTransform ActiveGun HasTarget)
  (set `self.Has Target` HasTarget)
  (bind _target_enemy (`self.Target Enemy`)
    (:`then`
      (set `self.TargetLocation` (`Actor.K2_GetActorLocation` _target_enemy)))
    (:`else`
      (bind _outhit (`KismetSystemLibrary.SphereTraceSingle` _returnvalue (+ _returnvalue (* (`Actor.GetActorForwardVector` _as_bp_the_gun_panda) 2000.0)) 50.0 "TraceTypeQuery1"))))
  (bind _returnvalue_2 (select `bool` (`self.Has Target`) :`false` (`.Location` (`GameplayStatics.BreakHitResult` _outhit)) :`true` (`self.TargetLocation`)))
  (bind _outhits (`KismetSystemLibrary.SphereTraceMultiForObjects` :`Start` _returnvalue_2 :`End` _returnvalue_2 :`Radius` (`self.AOERadius`) :`ObjectTypes` (`|MakeArray` "ObjectTypeQuery3" "ObjectTypeQuery2" :!type "EObjectTypeQuery Enum") :`DrawDebugType` "ForDuration" :`TraceColor` (struct :`G` 0.183846 :`B` 1.0 :`A` 1.0) :`TraceHitColor` (struct :`R` 1.0 :`G` 0.869988 :`A` 1.0) :`DrawTime` 0.5))
  (for _array_element _outhits
    (bind (_bblockinghit _binitialoverlap _time _distance _location _impactpoint _normal _impactnormal _physmat _hitactor _hitcomponent _hitbonename _bonename _hititem _elementindex _faceindex _tracestart) (`GameplayStatics.BreakHitResult` _array_element))
    (`KismetArrayLibrary.Array_AddUnique` (`self.Hit Actor`) _hitactor))
  (for _array_element_2 _hit_actor
    (`|ExecutionSequence`
      (:`then_0`
        (bind _returnvalue_3 (`Actor.GetComponentByClass` _array_element_2 "/Game/Topher/StatusEffectBPCs/BPC_StatusEffectManager.BPC_StatusEffectManager_C"))
        (if (`KismetSystemLibrary.IsValid` _returnvalue_3)
          (`/Game/Topher/StatusEffectBPCs/BPC_StatusEffectManager.AddStatus` _returnvalue_3 "NewEnumerator7" false)))
      (:`then_1`
        (if (`KismetSystemLibrary.DoesImplementInterface` _array_element_2 "/Game/Topher/GunInterface.GunInterface_C")
          (message `/Game/Topher/GunInterface.Pull` _array_element_2 _tracestart)))))
  (`KismetArrayLibrary.Array_Clear` _hit_actor))