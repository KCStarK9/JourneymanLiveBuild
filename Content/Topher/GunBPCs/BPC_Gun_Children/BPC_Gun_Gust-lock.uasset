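; Gust-lock gun component, a child gun Blueprint that fires a gust to push things in front of the Gun Panda.
; ShootGun runs the parent logic, then capsule-traces forward for Pawns and WorldDynamic objects.
; Trace length is the distance to the target, or without one comes from a forward sphere trace with a minimum length.
; Hit actors are de-duplicated, and those implementing GunInterface receive PushMessage with trace endpoints.
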(event `self.ShootGun`
  (params (TargetEnemy :type "Actor Object Reference") (MuzzleOneTransform :type "Transform Structure") (MuzzleTwoTransform :type "Transform Structure") (ActiveGun :type Integer) (HasTarget :type Boolean))
  (bind _hit_actor (`self.Hit Actor`))
  (bind _as_bp_the_gun_panda (`self.As BP The Gun Panda`))
  (bind _as_bp_the_gun_panda_2 (`self.As BP The Gun Panda`))
  (bind _returnvalue (`Actor.K2_GetActorLocation` _as_bp_the_gun_panda_2))
  (bind _returnvalue_2 (`Actor.K2_GetActorLocation` _as_bp_the_gun_panda))
  (`parent.ShootGun` TargetEnemy MuzzleOneTransform MuzzleTwoTransform ActiveGun HasTarget)
  (set `self.Has Target` HasTarget)
  (`self.Target Enemy`
    (:`then`
      _)
    (:`else`
      (bind _outhit (`KismetSystemLibrary.SphereTraceSingle` :`Start` _returnvalue_2 :`End` (+ _returnvalue_2 (* (`Actor.GetActorForwardVector` _as_bp_the_gun_panda) 2000.0)) :`Radius` 50.0 :`TraceChannel` "TraceTypeQuery1" :`DrawTime` 0.5))))
  (bind _outhits (`KismetSystemLibrary.CapsuleTraceMultiForObjects` :`Start` _returnvalue :`End` (+ _returnvalue (* (`Actor.GetActorForwardVector` _as_bp_the_gun_panda_2) (`KismetMathLibrary.SelectFloat` (`Actor.GetDistanceTo` (`self.As BP The Gun Panda`) (`self.Target Enemy`)) (`KismetMathLibrary.FMax` (`.Distance` (`GameplayStatics.BreakHitResult` _outhit)) 500.0) (`self.Has Target`)))) :`Radius` 100.0 :`HalfHeight` 90.0 :`ObjectTypes` (`|MakeArray` "ObjectTypeQuery3" "ObjectTypeQuery2" :!type "EObjectTypeQuery Enum") :`TraceColor` (struct :`G` 0.363212 :`B` 1.0 :`A` 1.0) :`TraceHitColor` (struct :`R` 1.0 :`G` 0.787746 :`A` 1.0) :`DrawTime` 0.5))
  (for _array_element _outhits
    (bind (_bblockinghit _binitialoverlap _time _distance _location _impactpoint _normal _impactnormal _physmat _hitactor _hitcomponent _hitbonename _bonename _hititem _elementindex _faceindex _tracestart _traceend) (`GameplayStatics.BreakHitResult` _array_element))
    (`KismetArrayLibrary.Array_AddUnique` (`self.Hit Actor`) _hitactor))
  (for _array_element_2 _hit_actor
    (if (`KismetSystemLibrary.DoesImplementInterface` _array_element_2 "/Game/Topher/GunInterface.GunInterface_C")
      (message `/Game/Topher/GunInterface.Push` _array_element_2 _tracestart _traceend)))
  (`KismetArrayLibrary.Array_Clear` _hit_actor))