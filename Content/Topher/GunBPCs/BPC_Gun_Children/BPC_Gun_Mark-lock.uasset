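; Mark-lock gun component, a child gun that damages its target and spreads a status effect to nearby pawns.
; After the parent shot logic, a valid target triggers basic and stagger damage through the enemy's BPC_Target component.
; A debug-drawn sphere trace at the target's location then adds a non-upgraded status to every hit actor with a status effect manager.
; CalculateDamage is left empty.
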(event `self.CalculateDamage`)

(event `self.ShootGun`
  (params (TargetEnemy :type "Actor Object Reference") (MuzzleOneTransform :type "Transform Structure") (MuzzleTwoTransform :type "Transform Structure") (ActiveGun :type Integer) (HasTarget :type Boolean))
  (bind ((`BasicDamage_37_C39876C24C3474862D83E7B52410AD6C` _basicdamage) (`StaggerDamage_39_E32A9290467E1174E0231C8FCB0181A0` _staggerdamage)) (break `/Game/Topher/Data/F_Gun` (`self.GunInfo`)))
  (bind _returnvalue (`Actor.GetComponentByClass` (`self.As Enemy Base`) "/Game/MainBlueprints/BPComponents/BPC_Target.BPC_Target_C"))
  (`parent.ShootGun` TargetEnemy MuzzleOneTransform MuzzleTwoTransform ActiveGun HasTarget)
  (bind _target_enemy (`self.Target Enemy`)
    (:`then`
      (`|ExecutionSequence`
        (:`then_0`
          (if (`KismetSystemLibrary.IsValid` _returnvalue)
            (`/Game/MainBlueprints/BPComponents/BPC_Target.Damage` _returnvalue _basicdamage _staggerdamage)))
        (:`then_1`
          (bind _returnvalue_2 (`Actor.K2_GetActorLocation` _target_enemy))
          (bind _outhits (`KismetSystemLibrary.SphereTraceMultiForObjects` :`Start` _returnvalue_2 :`End` _returnvalue_2 :`Radius` (`self.AOERadius`) :`ObjectTypes` (`|MakeArray` "ObjectTypeQuery3" :!type "EObjectTypeQuery Enum") :`DrawDebugType` "ForDuration" :`TraceColor` (struct :`G` 0.183846 :`B` 1.0 :`A` 1.0) :`TraceHitColor` (struct :`R` 1.0 :`G` 0.869988 :`A` 1.0) :`DrawTime` 0.5))
          (for _array_element _outhits
            (bind _returnvalue_3 (`Actor.GetComponentByClass` (`.HitActor` (`GameplayStatics.BreakHitResult` _array_element)) "/Game/Topher/StatusEffectBPCs/BPC_StatusEffectManager.BPC_StatusEffectManager_C"))
            (if (`KismetSystemLibrary.IsValid` _returnvalue_3)
              (`/Game/Topher/StatusEffectBPCs/BPC_StatusEffectManager.AddStatus` _returnvalue_3 "NewEnumerator8" false)))
          (set `self.Target Enemy` null)
          (set `self.Damage` 0.0)
          (set `self.Stagger` 0.0))))
    (:`else`)))